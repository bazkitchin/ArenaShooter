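; In-game player controller that spawns and possesses the player pawn, routes input to it, and swaps between HUD and death screen.
; BeginPlay and Respawn share one path, reusing the current pawn's transform or the game mode's spawn location.
; Movement, look, firing, skill and throttled use inputs pass through a validated pawn lookup.
; Spawning registers the character with the game instance and saves it to a name-based slot; loading is disabled.
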(event `self.ReceiveBeginPlay`
  (bind _returnvalue (`self.K2_GetPawn`))
  ;[1 1 1] Spawn the player at the start of the game and during respawn
  (`/Engine/EditorBlueprintResources/StandardMacros.IsValid` _returnvalue :!label _label
    (:`Is Valid`
      (set `self.RespawnTransform` (`self.GetTransform` _returnvalue))
      (`self.K2_DestroyActor` _returnvalue))
    (:`Is Not Valid`
      (bind _spawnpoint (`/Game/Blueprint/InGameMode.GetSpawnLocation` (cast `/Game/Blueprint/InGameMode` (`GameplayStatics.GetGameMode`) :!pure true)))
      (set `self.RespawnTransform` _spawnpoint)))
  (bind _returnvalue_2 (`|SpawnActorFromClass` "/Game/Blueprint/Characters/1_PlayerBase.1_PlayerBase_C" (`self.RespawnTransform`) "Undefined" "OverrideRootScale" null null))
  (`self.Possess` _returnvalue_2)
  (`self.SaveOrLoadCharacter`)
  (`self.ShowIngameHUD`))

(event `Respawn`
  ;[1 1 1] Spawn the player at the start of the game and during respawn
  (goto _label))

(event `ShowIngameHUD`
  ;[1 1 1] Show HUD and make it the game the players focus
  (set `self.bShowMouseCursor` false)
  (`WidgetBlueprintLibrary.SetFocusToGameViewport`)
  (`WidgetBlueprintLibrary.SetInputMode_GameOnly` self)
  (`WidgetLayoutLibrary.RemoveAllWidgets`)
  (bind _returnvalue (`|CreateWidget` "/Game/UMG/HUD.HUD_C" self))
  (bind _output_get (set `self.HUD` _returnvalue))
  (`UserWidget.AddToViewport` _output_get 0)
  (bind _as1_player_base (cast `/Game/Blueprint/Characters/1_PlayerBase` (`self.K2_GetPawn`)))
  (`/Game/Blueprint/Characters/1_PlayerBase.UpdateHUDHealth` _as1_player_base)
  (`/Game/Blueprint/Characters/1_PlayerBase.UpdateHUDXpBar` _as1_player_base))

(event `InputAxis|MoveForwards`
  (params (AxisValue :type "Float (single-precision)"))
  ;[1 1 1] Move character around using standard movement
  (bind _player (`self.GetPlayerPawn`)
    (:`Valid`
      (`Pawn.AddMovementInput` _player (`SceneComponent.GetForwardVector` (`Character.CapsuleComponent` _player)) AxisValue false))))

(event `InputAxis|RightMouse`
  (params (AxisValue :type "Float (single-precision)"))
  ;[1 1 1] Mouse buttons
  (if (> AxisValue 0.5)
    (bind _player (`self.GetPlayerPawn`)
      (:`Valid`
        (bind _as1_player_base (cast `/Game/Blueprint/Characters/1_PlayerBase` _player))
        (`/Game/Blueprint/Characters/1_PlayerBase.EventUseRightHand` _as1_player_base)))))

(event `InputAxis|MoveRight`
  (params (AxisValue :type "Float (single-precision)"))
  ;[1 1 1] Move character around using standard movement
  (bind _player (`self.GetPlayerPawn`)
    (:`Valid`
      (`Pawn.AddMovementInput` _player (`SceneComponent.GetRightVector` (`Character.CapsuleComponent` _player)) AxisValue false))))

(event `InputAxis|LeftMouse`
  (params (AxisValue :type "Float (single-precision)"))
  ;[1 1 1] Mouse buttons
  (if (> AxisValue 0.5)
    (bind _player (`self.GetPlayerPawn`)
      (:`Valid`
        (bind _as1_player_base (cast `/Game/Blueprint/Characters/1_PlayerBase` _player))
        (`/Game/Blueprint/Characters/0_BasePlayer.ShotGun` _as1_player_base)))))

(event `InputAxis|Jump`
  (params (AxisValue :type "Float (single-precision)"))
  ;[1 1 1] Move character around using standard movement
  (if (> AxisValue 0.5)
    (bind _player (`self.GetPlayerPawn`)
      (:`Valid`
        (`Character.Jump` _player)))))

(event `InputAxis|Use`
  (params (AxisValue :type "Float (single-precision)"))
  ;[1 1 1] Use key (default = 'e')
  (`|ExecutionSequence`
    (:`then_0`
      (if (> AxisValue 0.5)
        (`/Engine/EditorBlueprintResources/StandardMacros.DoOnce` false :!label _label_2
          (:`Completed`
            (bind _player (`self.GetPlayerPawn`)
              (:`Valid`
                (bind _as1_player_base (cast `/Game/Blueprint/Characters/1_PlayerBase` _player))
                (`/Game/Blueprint/Characters/1_PlayerBase.PerformUse` _as1_player_base)))))))
    (:`then_1`
      (`KismetSystemLibrary.Delay` 0.7)
      (goto _label_2 :!via `Reset`))))

(event `InputAxis|LookRight`
  (params (AxisValue :type "Float (single-precision)"))
  ;[1 1 1] Move character around using standard movement
  (bind _player (`self.GetPlayerPawn`)
    (:`Valid`
      (`Pawn.AddControllerYawInput` _player AxisValue))))

(event `InputAxis|LookUp`
  (params (AxisValue :type "Float (single-precision)"))
  ;[1 1 1] Move character around using standard movement
  (bind _player (`self.GetPlayerPawn`)
    (:`Valid`
      (`Pawn.AddControllerPitchInput` _player (* AxisValue -1.0)))))

(event `PlayerDied`
  ;[1 1 1] When player dies - spawn the death screen
  (`WidgetLayoutLibrary.RemoveAllWidgets`)
  (set `self.bShowMouseCursor` true)
  (bind _returnvalue (`|CreateWidget` "/Game/UMG/RespawnScreen.RespawnScreen_C" self))
  (`UserWidget.AddToViewport` _returnvalue 0))

(event `InputAction|SwitchToSkill1`
  (params (Key :type "Key Structure"))
  ;[1 1 1] Switch to skill based on keyboard
  (:`Pressed`
    (bind _player (`self.GetPlayerPawn`)
      (:`Valid`
        (bind _as1_player_base (cast `/Game/Blueprint/Characters/1_PlayerBase` _player))
        (`/Game/Blueprint/Characters/1_PlayerBase.SwitchToSkill` _as1_player_base 1)))))

(event `InputAction|SwitchToSkill2`
  (params (Key :type "Key Structure"))
  ;[1 1 1] Switch to skill based on keyboard
  (:`Pressed`
    (bind _player (`self.GetPlayerPawn`)
      (:`Valid`
        (bind _as1_player_base (cast `/Game/Blueprint/Characters/1_PlayerBase` _player))
        (`/Game/Blueprint/Characters/1_PlayerBase.SwitchToSkill` _as1_player_base 2)))))

(fn `LoadCharacter`
  (params (SlotName :type String))
  (locals (LSavedData :type "/Game/Blueprint/CharacterSave Object Reference") (PlayersPawn :type "/Game/Blueprint/Characters/1_PlayerBase Object Reference"))
  (bind _returnvalue (`GameplayStatics.LoadGameFromSlot` SlotName))
  (bind _ascharacter_save (cast `/Game/Blueprint/CharacterSave` _returnvalue)
    (:`then`
      (set `local.LSavedData` _ascharacter_save)
      (`|ExecutionSequence`
        (:`then_0`
          (bind _as1_player_base (cast `/Game/Blueprint/Characters/1_PlayerBase` (`self.K2_GetPawn`))
            (:`then`
              (set `local.PlayersPawn` _as1_player_base))
            (:`CastFailed`
              (return))))
        (:`then_1`
          (`/Game/Blueprint/Characters/1_PlayerBase.LoadDataFromSaveStruct` (`local.PlayersPawn`) (`/Game/Blueprint/CharacterSave.CharacterData` (`local.LSavedData`))))))
    (:`CastFailed`
      (return))))

(fn `SaveCharacter`
  (locals (LSaveData :type "/Game/Blueprint/CharacterSave Object Reference") (PlayerCharacter :type "/Game/Blueprint/Characters/1_PlayerBase Object Reference"))
  (`|ExecutionSequence`
    (:`then_0`
      (bind _returnvalue (`GameplayStatics.CreateSaveGameObject` "/Game/Blueprint/CharacterSave.CharacterSave_C"))
      (set `local.LSaveData` _returnvalue)
      (bind _as1_player_base (cast `/Game/Blueprint/Characters/1_PlayerBase` (`self.K2_GetPawn`))
        (:`then`
          (set `local.PlayerCharacter` _as1_player_base))
        (:`CastFailed`
          (return))))
    (:`then_1`
      (bind _datatosave (`/Game/Blueprint/Characters/1_PlayerBase.CopyDataIntoSaveStruct` (`local.PlayerCharacter`)))
      (set `/Game/Blueprint/CharacterSave.CharacterData` _datatosave (`local.LSaveData`))
      (`GameplayStatics.SaveGameToSlot` (`local.LSaveData`) (`.Name_3_53A02E294C6E495BFF5DFEB10A2EB126` (break `/Game/Blueprint/sCharacterSaveData` _datatosave)))
      (return))))

(fn `SaveOrLoadCharacter`
  (locals (LCharacter :type "/Game/Blueprint/Characters/1_PlayerBase Object Reference"))
  (bind _asmy_game_instance (cast `/Game/Blueprint/MyGameInstance` (`GameplayStatics.GetGameInstance`))
    (:`then`
      (bind _as1_player_base (cast `/Game/Blueprint/Characters/1_PlayerBase` (`self.K2_GetPawn`))
        (:`then`
          (set `local.LCharacter` _as1_player_base)
          (for _array_element (`/Game/Blueprint/MyGameInstance.ListOfCharacterSaves` _asmy_game_instance)
            (if (`KismetStringLibrary.EqualEqual_StrStr` _array_element (`/Game/Blueprint/Characters/1_PlayerBase.CharacterName` (`local.LCharacter`)))
              (`KismetSystemLibrary.PrintString` "Player loading disabled" true true (struct :`R` 1.0 :`G` 0.930123 :`B` 0.961061 :`A` 1.0) 5.0)))
          (bind _success (`/Game/Blueprint/MyGameInstance.CreateNewCharacter` _asmy_game_instance (`/Game/Blueprint/Characters/1_PlayerBase.CharacterName` (`local.LCharacter`))))
          (if _success
            (`self.SaveCharacter`)
            (`KismetSystemLibrary.PrintString` "Saving character")
            (else
              (`KismetSystemLibrary.PrintString` "Error: Saving character list"))))
        (:`CastFailed`
          (return))))
    (:`CastFailed`
      (return))))

(fn `UserConstructionScript`)