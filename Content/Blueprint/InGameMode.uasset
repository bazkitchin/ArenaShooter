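; In-game game mode that supplies spawn transforms, favoring player starts with no pawns nearby.
; BeginPlay caches the transform of every PlayerStart in SpawnPoints.
; GetSpawnLocation repeatedly picks a random cached point and sphere-traces it for pawns, with debug drawing on, returning the first clear one.
; Picks can repeat, and if every attempt is blocked it returns the last point tried, even though occupied.
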(event `self.ReceiveBeginPlay`
  (bind _outactors (`GameplayStatics.GetAllActorsOfClass` "/Script/Engine.PlayerStart"))
  (for _array_element _outactors
    (`KismetArrayLibrary.Array_Add` (`self.SpawnPoints`) (`self.GetTransform` _array_element))))

(fn `GetSpawnLocation`
  (returns (SpawnPoint :type "Transform Structure"))
  (locals (ValidSpawnPoint :type "Transform Structure"))
  (bind _spawnpoints (`self.SpawnPoints`))
  (bind _returnvalue (`KismetArrayLibrary.Array_Length` _spawnpoints))
  (for _ (range (+ _returnvalue 1))
    (bind _output_get (set `local.ValidSpawnPoint` (`|GetArrayItem` _spawnpoints (`KismetMathLibrary.RandomInteger` _returnvalue))))
    (bind _location (.location _output_get))
    (bind (_outhits _returnvalue_2) (`KismetSystemLibrary.SphereTraceMultiForObjects` :`Start` _location :`End` _location :`Radius` 200.0 :`ObjectTypes` (`|MakeArray` "ObjectTypeQuery3" :!type "EObjectTypeQuery Enum") :`DrawDebugType` "ForDuration"))
    (if (not _returnvalue_2)
      (return (`local.ValidSpawnPoint`))))
  (return (`local.ValidSpawnPoint`)))

(fn `UserConstructionScript`)