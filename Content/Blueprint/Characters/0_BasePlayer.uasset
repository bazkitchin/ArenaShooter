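; Base character class for players and AI, handling health, death, weapon hands and attack type, with stub events for child classes.
; Each Tick bobs the hand sockets during movement and aims them at the camera trace hit.
; Weapon use sets an attack type for the right hand only.
; Death notifies AI controllers, bursts particles in the random body colour and destroys the pawn, weapons and attached wind source.
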(event `self.ReceiveBeginPlay`
  ;[1 1 1] Saves the offset of the hands for later use
  (`|ExecutionSequence`
    (:`then_0`
      (set `self.RightHandOffset` (`SceneComponent.GetRelativeTransform` (`self.RightHandSocket`))))
    (:`then_1`
      (set `self.LeftHandOffset` (`SceneComponent.GetRelativeTransform` (`self.LeftHandSocket`))))
    (:`then_2`
      (`self.ResetToFullHealth`))
    (:`then_3`
      (bind _returnvalue (`|SpawnActorFromClass` "/Script/Engine.WindDirectionalSource" (`KismetMathLibrary.MakeTransform` (`self.K2_GetActorLocation`)) "Undefined" "OverrideRootScale" null null))
      (bind _output_get (set `self.BodyWind` _returnvalue))
      (`SceneComponent.K2_AttachToComponent` (`WindDirectionalSource.Component` _output_get) (`self.CapsuleComponent`) "None" "SnapToTarget" "KeepRelative" "KeepRelative" true)
      (`/Game/Blueprint/GeneralFunctions.UpdateWindActor` _output_get 200.0 200.0))))

(event `self.ReceiveTick`
  (params (DeltaSeconds :type "Float (single-precision)"))
  (bind _returnvalue (`self.K2_GetActorLocation`))
  (bind _lefthandsocket (`self.LeftHandSocket`))
  (bind _righthandsocket (`self.RightHandSocket`))
  (bind _returnvalue_2 (`SceneComponent.K2_GetComponentRotation` (`self.Camera`)))
  (bind _returnvalue_3 (not (== (`self.PreviousLocation`) _returnvalue)))
  (`|ExecutionSequence`
    (:`then_0`
      ;[1 1 1] If player is moving set the bob of the two hands
      (`self.HandBob` _returnvalue_3 (`self.RightHandOffset`) (`self.RightHandBob`) 7.5 -0.5 (`self.RightHandSocket`))
      (`self.HandBob` _returnvalue_3 (`self.LeftHandOffset`) (`self.LeftHandBob`) 7.5 0.5 (`self.LeftHandSocket`))
      (set `self.PreviousLocation` _returnvalue))
    (:`then_1`
      ;[1 1 1] When the controller moves up and down the hands follow
      (bind (_hit _somethinghit) (`self.LookingAt`))
      (if _somethinghit
        (bind (_bblockinghit _binitialoverlap _time _distance _location) (`GameplayStatics.BreakHitResult` _hit))
        (`SceneComponent.K2_SetWorldRotation` _lefthandsocket (`KismetMathLibrary.FindLookAtRotation` (`SceneComponent.K2_GetComponentLocation` _lefthandsocket) _location) false false)
        (`SceneComponent.K2_SetWorldRotation` _righthandsocket (`KismetMathLibrary.FindLookAtRotation` (`SceneComponent.K2_GetComponentLocation` _righthandsocket) _location) false false)
        (else
          (`SceneComponent.K2_SetWorldRotation` (`self.LeftHandSocket`) _returnvalue_2 false false)
          (`SceneComponent.K2_SetWorldRotation` (`self.RightHandSocket`) _returnvalue_2 false false))))
    (:`then_2`
      (set `self.PlayerAttackType` "NewEnumerator0"))))

(event `ShotGun`
  ;[1 1 1] Overriden by other classes
)

(event `KillEnemy`
  ;[1 1 1] Overriden by other classes
)

(event `/Game/Blueprint/Interfaces/iInteractive.AffectHealth`
  (params (Amount :type Integer) (`WhoDidThat?` :type "Actor Object Reference"))
  ;[1 1 1] Do this when character is hit/takes damage
  (bind _output_get (set `self.CurrentHealth` (- (`self.CurrentHealth`) Amount)))
  (if (<= _output_get 0)
    (`|ExecutionSequence`
      (:`then_0`
        (`/Engine/EditorBlueprintResources/StandardMacros.IsValid` `WhoDidThat?`
          (:`Is Valid`
            (bind _as0_base_player (cast `/Game/Blueprint/Characters/0_BasePlayer` `WhoDidThat?`))
            (`self.TargetLost` _as0_base_player)
            (`self.KillEnemy` _as0_base_player))))
      (:`then_2`
        (`self.Died`)))))

(event `Died`
  (bind (_r _g _b) (break `LinearColor` (`self.PlayerColour`)))
  ;[1 1 1] On character death do this
  (bind _returnvalue (`GameplayStatics.SpawnEmitterAtLocation` "/Game/ParticleSystems/P_CubeDeath.P_CubeDeath" (`self.K2_GetActorLocation`)))
  (`ParticleSystemComponent.SetVectorParameter` _returnvalue "PlayerColour" (`KismetMathLibrary.MakeVector` _r _g _b))
  (`self.TargetLost`)
  (`self.DestroyAllPlayerActors`))

(event `TargetLost`
  ;[1 1 1] If the target that was being shot at has gone
  (bind _asai_basic (cast `/Game/AI/AI_Basic` (`self.GetController`)))
  (`/Game/AI/AI_Basic.PawnDied` _asai_basic))

(event `ActuallyFiredRightHand`
  (bind _out_object (`/Game/Blueprint/GeneralMacros.IsValidReturn` (`self.RightHand`))
    (:`Is Valid`
      (`KismetSystemLibrary.PrintString` "Hello")
      (if (> (`/Game/Blueprint/Weapons/1_Weapon.Range` _out_object) 0.0)
        (bind _weaponhanded (`/Game/Blueprint/Items/0_Item.WeaponHanded` _out_object))
        (switch `/Game/Blueprint/Enumerations/eNumWeaponHanded` _weaponhanded
          (:`NewEnumerator0`
            (set `self.PlayerAttackType` "NewEnumerator5" :!label _label))
          (:`NewEnumerator1`
            (goto _label))
          (:`NewEnumerator2`
            (set `self.PlayerAttackType` "NewEnumerator9")))
        (else
          (switch `/Game/Blueprint/Enumerations/eNumWeaponHanded` _weaponhanded
            (:`NewEnumerator0`
              (set `self.PlayerAttackType` "NewEnumerator3" :!label _label_2))
            (:`NewEnumerator1`
              (goto _label_2))
            (:`NewEnumerator2`
              (set `self.PlayerAttackType` "NewEnumerator10"))))))))

(event `ActuallyFiredLeftHand`)

(event `WeaponHasBeenUsed`
  (params (Weapon :type "/Game/Blueprint/Weapons/1_Weapon Object Reference"))
  (if (== Weapon (`self.RightHand`))
    (`self.ActuallyFiredRightHand`)
    (else
      (`self.ActuallyFiredLeftHand`))))

(fn `AdjustShotForDifficulty`
  (params (Controller :type "Controller Object Reference"))
  (returns (AdjustmentVector :type "Vector Structure"))
  (locals (AIControlled :type Boolean) (Inaccurary :type "Vector Structure" :default (0.0 0.0 0.0)))
  (cast `AIController` Controller
    (:`then`
      (set `local.AIControlled` true)
      (bind _output_get (set `local.Inaccurary` (`KismetMathLibrary.MakeVector` 0.0 (`KismetMathLibrary.RandomFloatInRange` -500.0 500.0) (`KismetMathLibrary.RandomFloatInRange` -500.0 500.0))))
      (set `local.Inaccurary` _output_get))
    (:`CastFailed`
      (set `local.AIControlled` false)
      (set `local.Inaccurary` (0.0 0.0 0.0))))
  (return (`local.Inaccurary`)))

(fn `DestroyAllPlayerActors`
  (`|ExecutionSequence`
    (:`then_0`
      (`self.K2_DestroyActor`))
    (:`then_1`
      (`/Game/Blueprint/GeneralMacros.SafeDestroy` (`self.RightHand`)))
    (:`then_2`
      (`/Game/Blueprint/GeneralMacros.SafeDestroy` (`self.LeftHand`)))
    (:`then_3`
      (`/Game/Blueprint/GeneralMacros.SafeDestroy` (`self.BodyWind`)))))

(fn `HandBob`
  (params (`PlayerMoved?` :type Boolean) (OriginalTransform :type "Transform Structure") (PtrBobAmount :type "Float (double-precision) (by ref)") (BobRate :type "Float (double-precision)" :default 7.5) (BobAmount :type "Float (double-precision)" :default -1.0) (Socket :type "ArrowComponent Object Reference"))
  (bind _returnvalue (+ PtrBobAmount BobRate))
  (bind _returnvalue_2 (* (`KismetMathLibrary.DegSin` _returnvalue) BobAmount))
  (if `PlayerMoved?`
    (`|VariableSetRef` PtrBobAmount _returnvalue)
    (`SceneComponent.K2_AddLocalOffset` Socket (`KismetMathLibrary.MakeVector` _returnvalue_2 0.0 _returnvalue_2) false false)
    (else
      (`|VariableSetRef` PtrBobAmount)
      (`SceneComponent.K2_SetRelativeLocation` Socket (.location OriginalTransform) false false))))

(fn `LookingAt`
  (returns (Hit :type "HitResult Structure") (SomethingHit :type Boolean))
  (bind _camera (`self.Camera`))
  (bind _returnvalue (`SceneComponent.K2_GetComponentLocation` _camera))
  (bind (_outhit _returnvalue_2) (`KismetSystemLibrary.LineTraceSingle` :`Start` _returnvalue :`End` (+ _returnvalue (`KismetMathLibrary.GreaterGreater_VectorRotator` (`KismetMathLibrary.MakeVector` (`self.ViewingDistance`)) (`SceneComponent.K2_GetComponentRotation` _camera))) :`TraceChannel` "TraceTypeQuery1" :`DrawDebugType` "ForOneFrame"))
  (return _outhit _returnvalue_2))

(fn `ResetToFullHealth`
  (set `self.CurrentHealth` (`self.StartingHealth`)))

(fn `SpawnWeapon`
  (params (Weapon :type "/Game/Blueprint/Weapons/1_Weapon Class Reference") (Socket :type "ArrowComponent Object Reference") (PtrActor :type "/Game/Blueprint/Weapons/1_Weapon Object Reference (by ref)"))
  (bind _returnvalue (`|SpawnActorFromClass` Weapon (`KismetMathLibrary.MakeTransform` (.location (`SceneComponent.K2_GetComponentToWorld` Socket)) (.rotation (`SceneComponent.K2_GetComponentToWorld` Socket))) "AlwaysSpawn" "OverrideRootScale" null self null))
  (`|VariableSetRef` PtrActor _returnvalue)
  (`self.K2_AttachToComponent` _returnvalue Socket "None" "SnapToTarget" "SnapToTarget" "KeepWorld" true))

(fn `UserConstructionScript`
  (bind _mesh (`self.Mesh`))
  (bind _mesh_2 (`self.Mesh`))
  (bind _returnvalue (`PrimitiveComponent.CreateDynamicMaterialInstance` _mesh 0 (`PrimitiveComponent.GetMaterial` _mesh 0)))
  (bind _output_get (set `self.PlayerColour` (make `LinearColor` (`KismetMathLibrary.RandomFloat`) 0.2 (`KismetMathLibrary.RandomFloat`) 1.0)))
  (`MaterialInstanceDynamic.SetVectorParameterValue` _returnvalue "Base Color" _output_get)
  (`SceneComponent.K2_AttachToComponent` (`self.RightHandSocket`) _mesh_2 "RightHandSocket" "SnapToTarget" "SnapToTarget" "KeepRelative" true)
  (`SceneComponent.K2_AttachToComponent` (`self.LeftHandSocket`) _mesh_2 "LeftHandSocket" "SnapToTarget" "SnapToTarget" "KeepRelative" true))