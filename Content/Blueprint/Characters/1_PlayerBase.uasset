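; Base player character Blueprint that arms the player with a bolt pistol in the left hand and a power hammer in the right.
; On BeginPlay it spawns both weapons, snaps them to the Gun and RightHandSocket components, and hides those placeholder components.
; The ShotGun and EventUseRightHand events delegate to UseWeapon on the matching weapon, leaving attack behavior to the weapons themselves.
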(event `self.ReceiveBeginPlay`
  (bind _righthandsocket (`self.RightHandSocket`))
  (bind _gun (`self.Gun`))
  (`|ExecutionSequence`
    (:`then_0`
      (bind _returnvalue (`|SpawnActorFromClass` "/Game/Blueprint/Weapons/1_BoltPistol.1_BoltPistol_C" (`KismetMathLibrary.MakeTransform` (.location (`SceneComponent.K2_GetComponentToWorld` (`self.Gun`))) (.rotation (`SceneComponent.K2_GetComponentToWorld` (`self.Gun`)))) "AlwaysSpawn" "OverrideRootScale" null self null))
      (bind _output_get (set `self.LeftHand` _returnvalue))
      (`self.K2_AttachToComponent` _output_get _gun "None" "SnapToTarget" "SnapToTarget" "KeepWorld" true)
      (`SceneComponent.SetHiddenInGame` _gun true false)
      (`parent.ReceiveBeginPlay`))
    (:`then_1`
      (bind _returnvalue_2 (`|SpawnActorFromClass` "/Game/Blueprint/Weapons/1_PowerHammer.1_PowerHammer_C" (`KismetMathLibrary.MakeTransform` (.location (`SceneComponent.K2_GetComponentToWorld` (`self.RightHandSocket`))) (.rotation (`SceneComponent.K2_GetComponentToWorld` (`self.RightHandSocket`)))) "AlwaysSpawn" "OverrideRootScale" null self null))
      (bind _output_get_2 (set `self.RightHand` _returnvalue_2))
      (`self.K2_AttachToComponent` _output_get_2 _righthandsocket "None" "SnapToTarget" "SnapToTarget" "KeepWorld" true)
      (`SceneComponent.SetHiddenInGame` _righthandsocket true false))))

(event `self.ShotGun`
  (`/Game/Blueprint/Weapons/0_Weapon.UseWeapon` (`self.LeftHand`)))

(event `EventUseRightHand`
  (`/Game/Blueprint/Weapons/0_Weapon.UseWeapon` (`self.RightHand`)))

(fn `UserConstructionScript`
  (`parent.UserConstructionScript`))