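; Base AI character that spawns weapons into both hands and can fire the right-hand one.
; BeginPlay records the starting location, then SpawnAIWeapon maps each hand's weapon choice to a bolt pistol, power hammer or none and spawns valid classes on that hand's socket.
; Tick pitches the right-hand socket to follow control rotation, and the ShotGun event triggers the right-hand weapon's use.
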(event `self.ReceiveBeginPlay`
  (`parent.ReceiveBeginPlay`)
  (set `self.StartingLocation` (`self.K2_GetActorLocation`))
  (`self.SpawnAIWeapon` (`self.InRightHand`) (`self.RightHandSocket`) (`self.RightHand`))
  (`self.SpawnAIWeapon` (`self.InLeftHand`) (`self.LeftHandSocket`) (`self.LeftHand`)))

(event `self.ReceiveTick`
  (params (DeltaSeconds :type "Float (single-precision)"))
  (`parent.ReceiveTick` DeltaSeconds)
  (`SceneComponent.K2_SetRelativeRotation` (`self.RightHandSocket`) (`KismetMathLibrary.MakeRotator` 0.0 (.pitch (`self.GetControlRotation`))) false false))

(event `ShotGun`
  (`/Game/Blueprint/Weapons/0_Weapon.UseWeapon` (`self.RightHand`)))

(fn `SpawnAIWeapon`
  (params (Weapon :type "/Game/Blueprint/eAIWeaponList Enum" :default "NewEnumerator2") (Socket :type "ArrowComponent Object Reference") (PtrActor :type "/Game/Blueprint/Weapons/0_Weapon Object Reference (by ref)"))
  (locals (LWeapon :type "/Game/Blueprint/Weapons/0_Weapon Class Reference" :default null))
  (bind _lweapon (`local.LWeapon`))
  (`|ExecutionSequence`
    (:`then_0`
      (switch `/Game/Blueprint/eAIWeaponList` Weapon
        (:`NewEnumerator2`
          (set `local.LWeapon` null))
        (:`NewEnumerator0`
          (set `local.LWeapon` "/Game/Blueprint/Weapons/1_BoltPistol.1_BoltPistol_C"))
        (:`NewEnumerator1`
          (set `local.LWeapon` "/Game/Blueprint/Weapons/1_PowerHammer.1_PowerHammer_C"))))
    (:`then_1`
      ;[1 1 1] If the class if a valid one spawn it
      (if (`KismetSystemLibrary.IsValidClass` _lweapon)
        (`self.SpawnWeapon` _lweapon Socket PtrActor)))))

(fn `UserConstructionScript`
  (`parent.UserConstructionScript`))