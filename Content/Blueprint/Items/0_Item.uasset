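; Base pickup item actor that toggles between lying on the floor as a physics mesh and being carried by a holder.
; Tick drives a custom-depth stencil highlight when the player is in range, and a name widget while a per-frame look-at flag is refreshed.
; Pickup hides and attaches it, registering player pickups with MyGameInstance; dropping places it in front of the holder.
; Equip and unequip call empty ShowItem/HideItem events.
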(event `self.ReceiveBeginPlay`
  (`self.Initialise`)
  (`/Engine/EditorBlueprintResources/StandardMacros.IsValid` (`self.Holder`)
    (:`Is Not Valid`
      (`self.ItemPutOnFloor`))))

(event `self.ReceiveTick`
  (params (DeltaSeconds :type "Float (single-precision)"))
  (`self.HighlightItem`))

(event `/Game/Blueprint/Interfaces/iPlayerInteraction.BeingLookedAt`
  (params (ByWhom :type "Actor Object Reference"))
  ;[1 1 1] Check if item is being looked at (needs to be refreshed every tick)
  (set `self.PlayerLookingAt` true))

(event `/Game/Blueprint/Interfaces/iPlayerInteraction.PlayerUsedMe`
  (params (ByWhom :type "Actor Object Reference"))
  (`self.PickedUp` ByWhom)
  (`self.IsPlayersPawn` ByWhom
    (:`IsPlayersPawn`
      (bind _asmy_game_instance (cast `/Game/Blueprint/MyGameInstance` (`GameplayStatics.GetGameInstance`)))
      (`/Game/Blueprint/MyGameInstance.GivePlayerItem` _asmy_game_instance self))))

(event `self.HighlightRange.OnComponentBeginOverlap`
  (params (OverlappedComponent :type "PrimitiveComponent Object Reference") (OtherActor :type "Actor Object Reference") (OtherComp :type "PrimitiveComponent Object Reference") (OtherBodyIndex :type Integer) (bFromSweep :type Boolean) (SweepResult :type "HitResult Structure (by ref)"))
  ;[1 1 1] When the player enters/leaves the highlight radius
  (`self.IsPlayersPawn` OtherActor
    (:`IsPlayersPawn`
      (set `self.PlayerInHighlightRadius` true))))

(event `self.HighlightRange.OnComponentEndOverlap`
  (params (OverlappedComponent :type "PrimitiveComponent Object Reference") (OtherActor :type "Actor Object Reference") (OtherComp :type "PrimitiveComponent Object Reference") (OtherBodyIndex :type Integer))
  ;[1 1 1] When the player enters/leaves the highlight radius
  (`self.IsPlayersPawn` OtherActor
    (:`IsPlayersPawn`
      (set `self.PlayerInHighlightRadius` false))))

(event `ShowItem`)

(event `HideItem`)

(event `EquipItem`
  (params (EquippedIndex :type Integer))
  (`self.ShowItem`)
  (set `self.Equipped?` true))

(event `UnequipItem`
  (`self.HideItem`)
  (set `self.Equipped?` false))

(fn `AddHighlight`
  (bind _pickupmesh (`self.PickUpMesh`))
  (`PrimitiveComponent.SetRenderCustomDepth` _pickupmesh true)
  (`PrimitiveComponent.SetCustomDepthStencilValue` _pickupmesh 1))

(fn `HighlightItem`
  (bind _pickuptext (`self.PickupText`))
  (bind _pickuptext_2 (`self.PickupText`))
  (if (`self.ItemIsOnFloor`)
    (`|ExecutionSequence` :!label _label
      (:`then_0`
        ;[1 1 1] If the player is within the highlight range the object is highlighted
        (if (`self.PlayerInHighlightRadius`)
          (`self.AddHighlight`)
          (else
            (`self.RemoveHighlight`))))
      (:`then_1`
        ;[1 1 1] If the players crosshair is looking at the object it puts the items name above it
        (if (`self.PlayerLookingAt`)
          (`/Engine/EditorBlueprintResources/StandardMacros.IsValid` _pickuptext
            (:`Is Valid`
              _)
            (:`Is Not Valid`
              (bind _returnvalue (`|CreateWidget` "/Game/UMG/PickText.PickText_C" (`GameplayStatics.GetPlayerController` 0) self))
              (bind _output_get (set `self.PickupText` _returnvalue))
              (`UserWidget.AddToViewport` _output_get 0)))
          (`/Game/UMG/PickText.Update` _pickuptext)
          (else
            (`/Engine/EditorBlueprintResources/StandardMacros.IsValid` _pickuptext_2
              (:`Is Valid`
                (`Widget.RemoveFromParent` _pickuptext_2)
                (`/Game/UMG/PickText.Destroy` _pickuptext_2))
              (:`Is Not Valid`
                _))
            (set `self.PickupText` null)))
        (set `self.PlayerLookingAt` false)))
    (else
      (`|ExecutionSequence`
        (:`then_0`
          (set `self.PlayerLookingAt` false))
        (:`then_1`
          (set `self.PlayerInHighlightRadius` false))
        (:`then_2`
          (goto _label))))))

(fn `Initialise`
  (`|ExecutionSequence`
    (:`then_0`
      (set `self.PlayerLookingAt` false))))

(fn `ItemPutOnFloor`
  (bind _pickupmesh (`self.PickUpMesh`))
  (bind _holder (`self.Holder`))
  (bind _returnvalue (+ (`self.K2_GetActorLocation` _holder) (`KismetMathLibrary.GreaterGreater_VectorRotator` (100.0 0.0 0.0) (`self.K2_GetActorRotation` _holder))))
  (`|ExecutionSequence`
    (:`then_0`
      (set `self.ItemIsOnFloor` true)
      (`self.HideItem`))
    (:`then_1`
      (`SceneComponent.SetVisibility` _pickupmesh true false)
      (`PrimitiveComponent.SetCollisionEnabled` _pickupmesh "QueryAndPhysics")
      (`PrimitiveComponent.SetSimulatePhysics` (`self.PickUpMesh`) true))
    (:`then_2`
      (`self.HighlightItem`))
    (:`then_3`
      (if (`self.Constructed`)
        (`/Engine/EditorBlueprintResources/StandardMacros.IsValid` _holder
          (:`Is Valid`
            (`self.K2_DetachFromActor` "KeepRelative")
            (`self.K2_SetActorLocation` _returnvalue false true)
            (`SceneComponent.K2_SetWorldLocation` (`self.PickUpMesh`) _returnvalue false true)
            (set `self.Holder` null)))))))

(fn `PickedUp`
  (params (`By Whom?` :type "Actor Object Reference"))
  (bind _pickupmesh (`self.PickUpMesh`))
  (`|ExecutionSequence`
    (:`then_0`
      (set `self.ItemIsOnFloor` false))
    (:`then_1`
      (set `self.PlayerInHighlightRadius` false))
    (:`then_2`
      (set `self.PlayerLookingAt` false))
    (:`then_3`
      (`SceneComponent.SetVisibility` _pickupmesh false false)
      (`PrimitiveComponent.SetSimulatePhysics` _pickupmesh false)
      (`PrimitiveComponent.SetCollisionEnabled` _pickupmesh "NoCollision"))
    (:`then_4`
      (`self.HighlightItem`))
    (:`then_5`
      (bind _output_get (set `self.Holder` `By Whom?`))
      (`self.K2_AttachToActor` _output_get "None" "SnapToTarget" "SnapToTarget" "KeepRelative"))))

(fn `RemoveHighlight`
  (`PrimitiveComponent.SetRenderCustomDepth` (`self.PickUpMesh`) false))

(fn `UserConstructionScript`
  (`SphereComponent.SetSphereRadius` (`self.HighlightRange`) (`self.HighlightRadius`) true)
  (`self.ItemPutOnFloor`)
  (set `self.Constructed` true))