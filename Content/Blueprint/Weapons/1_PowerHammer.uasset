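; Power hammer melee weapon Blueprint that swings and then applies an area health effect around its wielder.
; MeleeStrike starts the swing, and Tick rotates the Cylinder by frame time, cancelling it when Recharge equals one.
; Near ninety degrees the rotation resets and a sphere trace at the Benefactor, ignoring it, calls AffectHealth on hit actors implementing iInteractive.
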(event `self.ReceiveTick`
  (params (DeltaSeconds :type "Float (single-precision)"))
  (bind _benefactor (`self.Benefactor`))
  (bind _returnvalue (`self.K2_GetActorLocation` _benefactor))
  (bind _returnvalue_2 (* -1000.0 (`GameplayStatics.GetWorldDeltaSeconds`)))
  (`parent.ReceiveTick` DeltaSeconds)
  (if (== (`self.Recharge%`) 1.0)
    (set `self.Swinging` false))
  (if (`self.Swinging`)
    (bind _output_get (set `self.SwingAngle` (+ (`self.SwingAngle`) _returnvalue_2)))
    (if (> _output_get -90.0)
      (`SceneComponent.K2_AddLocalRotation` (`self.Cylinder`) (`KismetMathLibrary.MakeRotator` 0.0 _returnvalue_2) false false)
      (else
        (set `self.SwingAngle` 0.0)
        (set `self.Swinging` false)
        (`SceneComponent.K2_SetRelativeRotation` :`self` (`self.Cylinder`))
        (bind _outhits (`KismetSystemLibrary.SphereTraceMulti` _returnvalue _returnvalue 200.0 "TraceTypeQuery1" false (`|MakeArray` _benefactor)))
        (for _array_element _outhits
          (bind _asi_interactive (cast `/Game/Blueprint/iInteractive` (`.HitActor` (`GameplayStatics.BreakHitResult` _array_element))))
          (`/Game/Blueprint/iInteractive.AffectHealth` _asi_interactive 100 (`self.Benefactor`)))))
    (else
      (`SceneComponent.K2_SetRelativeRotation` :`self` (`self.Cylinder`)))))

(event `self.MeleeStrike`
  (set `self.Swinging` true))

(fn `UserConstructionScript`
  (`parent.UserConstructionScript`))