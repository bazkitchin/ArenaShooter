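; Base weapon Blueprint that handles firing, cooldown, sound and mesh visibility.
; UseWeapon fires once the Tick-driven cooldown reaches AttackRate, otherwise calls an empty NotReadyYet event.
; Positive Range means ranged: either a projectile actor with an impulse, or a particle-backed hitscan trace dealing random damage through iInteractive.
; Zero or negative Range calls an empty MeleeStrike event, and WhereIsWeaponPointing exposes an aim trace.
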(event `self.ReceiveBeginPlay`
  (`parent.ReceiveBeginPlay`)
  (`self.CalculateRefireRate`)
  (`self.CooldownWeapon` 120.0)
  (`AudioComponent.SetSound` (`self.FireSound`) (`self.AttackSound`)))

(event `self.ReceiveTick`
  (params (DeltaSeconds :type "Float (single-precision)"))
  (`parent.ReceiveTick` DeltaSeconds)
  (`self.CooldownWeapon` DeltaSeconds))

(event `UseWeapon`
  (`self.CanFire?`
    (:`Fire`
      (`self.FireWeapon`)
      (`self.ResetCooldown`))
    (:`CannotFire`
      (`self.NotReadyYet`))))

(event `FireWeapon`
  (`AudioComponent.Play` (`self.FireSound`) 0.0)
  (`self.RangedWeapon?`
    (:`Ranged`
      (if (`self.ProjectileParticle?`)
        (`self.SpawnProjectileParticle`)
        (else
          (`self.SpawnProjectile`))))
    (:`Melee`
      (`self.MeleeStrike`))))

(event `NotReadyYet`)

(event `MeleeStrike`)

(event `self.ShowItem`
  ;[1 1 1] Show and hide the Weapon Mesh
  (`SceneComponent.SetHiddenInGame` (`self.WeaponMesh`) false false))

(event `self.HideItem`
  ;[1 1 1] Show and hide the Weapon Mesh
  (`SceneComponent.SetHiddenInGame` (`self.WeaponMesh`) true false))

(fn `CalculateRefireRate`
  (set `self.RefireTime` (/ (`self.AttackRate`) 1.0)))

(fn `CooldownWeapon`
  (params (TimeDelta :type "Float (double-precision)"))
  (bind _output_get (set `self.Cooldown` (`KismetMathLibrary.FClamp` (+ TimeDelta (`self.Cooldown`)) 0.0 (`self.RefireTime`))))
  (set `self.Recharge%` (/ _output_get (`self.RefireTime`))))

(fn `ResetCooldown`
  (set `self.Cooldown` 0.0)
  (set `self.Recharge%` 0.0))

(fn `SpawnProjectile`
  (bind _barrel (`self.Barrel`))
  (bind _rotation (.rotation (`SceneComponent.K2_GetComponentToWorld` _barrel)))
  (`|SpawnActorFromClass` (`self.ProjectileActor`) (`KismetMathLibrary.MakeTransform` (+ (.location (`SceneComponent.K2_GetComponentToWorld` _barrel)) (`KismetMathLibrary.GreaterGreater_VectorRotator` (`self.InitialProjectileOffset`) _rotation)) _rotation) "AlwaysSpawn" "OverrideRootScale" null 2.0 (`KismetMathLibrary.GreaterGreater_VectorRotator` (`self.InitialForce`) (`SceneComponent.K2_GetComponentRotation` _barrel)) (`self.Benefactor`) null))

(fn `SpawnProjectileParticle`
  (bind _returnvalue (`SceneComponent.K2_GetComponentLocation` (`self.Barrel`)))
  (bind _returnvalue_2 (+ _returnvalue (`KismetMathLibrary.GreaterGreater_VectorRotator` (`KismetMathLibrary.MakeVector` (`self.Range`)) (`SceneComponent.K2_GetComponentRotation` (`self.Barrel`)))))
  (`GameplayStatics.SpawnEmitterAtLocation` (`self.ProjectileEffect`) _returnvalue (`KismetMathLibrary.FindLookAtRotation` _returnvalue _returnvalue_2))
  (bind (_outhit _returnvalue_3) (`KismetSystemLibrary.LineTraceSingle` _returnvalue _returnvalue_2 "TraceTypeQuery1"))
  (if _returnvalue_3
    (bind (_bblockinghit _binitialoverlap _time _distance _location _impactpoint _normal _impactnormal _physmat _hitactor) (`GameplayStatics.BreakHitResult` _outhit))
    (`GameplayStatics.SpawnEmitterAtLocation` "/Game/ParticleSystems/P_BulletImpact.P_BulletImpact" _location)
    (bind (_asi_interactive _bsuccess) (cast `/Game/Blueprint/Interfaces/iInteractive` _hitactor :!pure true))
    (if _bsuccess
      (`/Game/Blueprint/Interfaces/iInteractive.AffectHealth` _asi_interactive (`KismetMathLibrary.RandomIntegerInRange` (`self.MinDamage`) (`self.MaxDamage`)) (`self.Benefactor`)))))

(fn `UserConstructionScript`
  (`parent.UserConstructionScript`))

(fn `WhereIsWeaponPointing`
  (params (`Debug?` :type Boolean))
  (returns (SomethingInRange :type Boolean) (PointingAtLocation :type "Vector Structure") (PointAtActor :type "Actor Object Reference"))
  (bind _barrel (`self.Barrel`))
  (bind _returnvalue (`SceneComponent.K2_GetComponentLocation` _barrel))
  (bind (_outhit _returnvalue_2) (`KismetSystemLibrary.LineTraceSingle` :`Start` _returnvalue :`End` (+ _returnvalue (`KismetMathLibrary.GreaterGreater_VectorRotator` (`KismetMathLibrary.MakeVector` (`self.Range`)) (`SceneComponent.K2_GetComponentRotation` _barrel))) :`TraceChannel` "TraceTypeQuery1" :`DrawDebugType` (select `bool` `Debug?` :`true` "ForDuration" :!type "EDrawDebugTrace Enum")))
  (bind (_bblockinghit _binitialoverlap _time _distance _location _impactpoint _normal _impactnormal _physmat _hitactor) (`GameplayStatics.BreakHitResult` _outhit))
  (return _returnvalue_2 _location _hitactor))