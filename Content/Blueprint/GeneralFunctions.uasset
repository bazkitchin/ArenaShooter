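; GeneralFunctions is a collection of shared helper functions for item-style rarity colours and wind actor setup.
; GetColourBasedOnRarity maps a rarity tier, from Broken to Unique, to a fixed colour.
; UpdateWindActor turns a given wind directional source into a point wind with the supplied radius, using one Strength value for speed, strength and maximum gust, with minimum gust zeroed.
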(fn `GetColourBasedOnRarity`
  (params (Rarity :type "/Game/Blueprint/Enumerations/eRarity Enum" :default "NewEnumerator0"))
  (returns (Colour :type "LinearColor Structure"))
  (locals (LocalColour :type "LinearColor Structure"))
  (`|ExecutionSequence`
    (:`then_0`
      (switch `/Game/Blueprint/Enumerations/eRarity` Rarity
        (:`NewEnumerator0`
          (set `local.LocalColour` (struct :`R` 0.140625 :`G` 0.140625 :`B` 0.140625 :`A` 1.0)))
        (:`NewEnumerator1`
          (set `local.LocalColour` (struct :`R` 1.0 :`G` 1.0 :`B` 1.0 :`A` 1.0)))
        (:`NewEnumerator2`
          (set `local.LocalColour` (struct :`G` 0.706272 :`B` 0.755208 :`A` 1.0)))
        (:`NewEnumerator3`
          (set `local.LocalColour` (struct :`G` 0.755208 :`B` 0.02189 :`A` 1.0)))
        (:`NewEnumerator4`
          (set `local.LocalColour` (struct :`R` 0.515625 :`G` 0.429693 :`A` 1.0)))))
    (:`then_1`
      (return (`local.LocalColour`)))))

(fn `UpdateWindActor`
  (params (In_Wind :type "WindDirectionalSource Object Reference") (Radius :type "Float (double-precision)") (Strength :type "Float (double-precision)"))
  (bind _component (`WindDirectionalSource.Component` In_Wind))
  (`|ExecutionSequence`
    (:`then_0`
      (`WindDirectionalSourceComponent.SetWindType` _component "Point"))
    (:`then_1`
      (`WindDirectionalSourceComponent.SetRadius` _component Radius))
    (:`then_2`
      (`WindDirectionalSourceComponent.SetSpeed` _component Strength))
    (:`then_3`
      (`WindDirectionalSourceComponent.SetStrength` _component Strength))
    (:`then_4`
      (`WindDirectionalSourceComponent.SetMaximumGustAmount` _component Strength))
    (:`then_5`
      (`WindDirectionalSourceComponent.SetMinimumGustAmount` _component 0.0))
    (:`then_6`
      (return))))