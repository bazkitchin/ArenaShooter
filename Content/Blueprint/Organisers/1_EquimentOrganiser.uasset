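; Equipment organiser that manages the player's equipped items in a fixed set of type-restricted slots.
; AddItem finds slots matching the item type, fills a free one or displaces the occupant, and empties paired slots for strict two-handed weapons.
; Overridden menu options unequip to the character stash, drop, or sell/store depending on environment, notifying the GameInstance that equipment has changed.
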(event `self.InitialiseStash`
  (params (NumberOfSlots :type Integer) (ListOfItemInInventory :type "Array of /Game/UMG/ItemInInventory Object Reference (by ref)"))
  ;[1 1 1] Manually set up the stash
  (set `self.Stash` (`|MakeArray` (make `/Game/Blueprint/Structures/sStashSlot` :`AllowedItems` "NewEnumerator0") (make `/Game/Blueprint/Structures/sStashSlot` :`Index` 1 :`AllowedItems` "NewEnumerator1") (make `/Game/Blueprint/Structures/sStashSlot` :`Index` 2 :`AllowedItems` "NewEnumerator2") (make `/Game/Blueprint/Structures/sStashSlot` :`Index` 3 :`AllowedItems` "NewEnumerator3") (make `/Game/Blueprint/Structures/sStashSlot` :`Index` 4 :`AllowedItems` "NewEnumerator4") (make `/Game/Blueprint/Structures/sStashSlot` :`Index` 5 :`AllowedItems` "NewEnumerator5") (make `/Game/Blueprint/Structures/sStashSlot` :`Index` 6 :`AllowedItems` "NewEnumerator8") (make `/Game/Blueprint/Structures/sStashSlot` :`Index` 7 :`AllowedItems` "NewEnumerator6") (make `/Game/Blueprint/Structures/sStashSlot` :`Index` 8 :`AllowedItems` "NewEnumerator8") (make `/Game/Blueprint/Structures/sStashSlot` :`Index` 9 :`AllowedItems` "NewEnumerator7") (make `/Game/Blueprint/Structures/sStashSlot` :`Index` 10 :`AllowedItems` "NewEnumerator7")))
  (for (_array_element _array_index) ListOfItemInInventory
    (`self.LinkStashSlotToItemInventory` _array_element _array_index)))

(event `self.TopOption`
  (params (Item :type "/Game/Blueprint/Items/0_Item Object Reference") (Index :type Integer))
  (bind ((`Item_12_C84B26924C9C7F00ADB80AB6ED8ACEAE` _item)) (break `/Game/Blueprint/Structures/sStashSlot` (`|GetArrayItem` (`self.Stash`) Index)))
  ;[1 1 1] Overload the equip to be unequip which clear the slot and place the item in the players stash
  (`/Game/Blueprint/Items/0_Item.UnequipItem` _item)
  (`self.AddItem` (`/Game/Blueprint/MyGameInstance.CharacterStash` (`self.GameInstance`)) _item 0)
  (`|ExecutionSequence`
    (:`then_0`
      (`self.ClearIndex` Index))
    (:`then_1`
      (`/Game/Blueprint/MyGameInstance.EquipmentHasChanged` (`self.GameInstance`)))))

(event `self.MiddleOption`
  (params (Index :type Integer))
  ;[1 1 1] Add the fact the equipment has changed once the player has dropped an item from their equipment
  (`/Game/Blueprint/Items/0_Item.UnequipItem` (`.Item_12_C84B26924C9C7F00ADB80AB6ED8ACEAE` (break `/Game/Blueprint/Structures/sStashSlot` (`|GetArrayItem` (`self.Stash`) Index))))
  (`/Game/Blueprint/MyGameInstance.EquipmentHasChanged` (`self.GameInstance`))
  (`parent.MiddleOption` Index))

(event `self.BottomOption`
  (params (Index :type Integer))
  ;[1 1 1] Add the fact the equipment has changed once the player has sold an item from their equipment
  (`parent.BottomOption` Index)
  (`/Game/Blueprint/Items/0_Item.UnequipItem` (`.Item_12_C84B26924C9C7F00ADB80AB6ED8ACEAE` (break `/Game/Blueprint/Structures/sStashSlot` (`|GetArrayItem` (`self.Stash`)))))
  (`/Game/Blueprint/MyGameInstance.EquipmentHasChanged` (`self.GameInstance`)))

(event `self.SetOptions`
  (params (Environment :type "/Game/Blueprint/Enumerations/eTypesOfStash Enum" :default "NewEnumerator0"))
  ;[1 1 1] Overload the text so it say the right thing
  (switch `/Game/Blueprint/Enumerations/eTypesOfStash` Environment
    (:`NewEnumerator0`
      (`self.SetOptionText` "Unequip Item" "Drop Item" "Not Available" true true))
    (:`NewEnumerator2`
      (`self.SetOptionText` "Unequip Item" "Drop Item" "Sell Item" true true true))
    (:`NewEnumerator3`
      (`self.SetOptionText` "Unequip Item" "Drop Item" "Store Item" true true true))))

(fn `AddItem`
  (params (Item :type "/Game/Blueprint/Items/0_Item Object Reference") (SlotIndex :type Integer))
  (returns (`Accepted?` :type Boolean) (DisplacedItem1 :type "/Game/Blueprint/Items/0_Item Object Reference") (DisplacedItem2 :type "/Game/Blueprint/Items/0_Item Object Reference"))
  (locals (CompatibleSlots :type "Array of Integer") (NewItem :type "/Game/Blueprint/Items/0_Item Object Reference") (OldItem1 :type "/Game/Blueprint/Items/0_Item Object Reference") (OldItem2 :type "/Game/Blueprint/Items/0_Item Object Reference") (Index :type Integer) (UseSlot0 :type Boolean :default true) (ItemIndex :type Integer) (`StrictTwoHanded?` :type Boolean))
  (bind _output (`|GetArrayItem` (`self.Stash`) (`local.Index`)))
  (bind _output_2 (`|GetArrayItem` (`self.Stash`) (`local.Index`)))
  (bind _output_3 (`|GetArrayItem` (`local.CompatibleSlots`)))
  (bind _output_4 (`|GetArrayItem` (`self.Stash`) _output_3))
  (`|ExecutionSequence`
    (:`then_0`
      (bind _output_get (set `local.NewItem` Item))
      (`/Game/Blueprint/GeneralMacros.IsValidReturn` _output_get
        (:`Is Not Valid`
          (return false null null))))
    (:`then_1`
      ;[1 1 1] Find all slot index that are compatible
      (for (_array_element _array_index) (`self.Stash`)
        (if (`|EnumEquality` (`.AllowedItems_20_2B0959BE43A9D2C413EE28A6C752CCC0` (break `/Game/Blueprint/Structures/sStashSlot` _array_element)) (`/Game/Blueprint/Items/0_Item.Type` (`local.NewItem`)))
          (`KismetArrayLibrary.Array_Add` (`local.CompatibleSlots`) _array_index))))
    (:`then_2`
      ;[1 1 1] If none were found, then the item cannot be equipped
      (switch `int` (`KismetArrayLibrary.Array_Length` (`local.CompatibleSlots`))
        (:`Default`
          (return false (`local.NewItem`) null))
        (:`0`
          (return false (`local.NewItem`) null))
        (:`1`
          ;[1 1 1] Check if any of the available slot are free, if not populate the first one, removing anything that was there before
          (for _array_element_2 (`local.CompatibleSlots`) :!label _label
            (bind _output_5 (`|GetArrayItem` (`self.Stash`) _array_element_2))
            (if (not (`.Full?_11_AC9CC015470371E7BC599091DAFEB896` (break `/Game/Blueprint/Structures/sStashSlot` _output_5)))
              (set `local.ItemIndex` _array_element_2)
              (bind _structout (setmembers `/Game/Blueprint/Structures/sStashSlot` :`StructRef` _output_5 :`Full?` true :`Item` (`local.NewItem`)))
              (`KismetArrayLibrary.Array_Set` (`self.Stash`) (`local.ItemIndex`) _structout)
              (set `local.UseSlot0` false)
              (break)))
          (if (`local.UseSlot0`)
            (set `local.ItemIndex` _output_3)
            (set `local.OldItem1` (`.Item_12_C84B26924C9C7F00ADB80AB6ED8ACEAE` (break `/Game/Blueprint/Structures/sStashSlot` _output_4)))
            (bind _structout_2 (setmembers `/Game/Blueprint/Structures/sStashSlot` :`StructRef` _output_4 :`Full?` true :`Item` (`local.NewItem`)))
            (`KismetArrayLibrary.Array_Set` (`self.Stash`) (`local.ItemIndex`) _structout_2)))
        (:`2`
          ;[1 1 1] If the new item or old one is strict two handed all slots need to be emptied
          (`|ExecutionSequence`
            (:`then_0`
              (set `local.StrictTwoHanded?` (`|EnumEquality` (`/Game/Blueprint/Items/0_Item.WeaponHanded` (`local.NewItem`)) "NewEnumerator2")))
            (:`then_1`
              (if (not (`local.StrictTwoHanded?`))
                (bind _out_object (`/Game/Blueprint/GeneralMacros.IsValidReturn` (`.Item_12_C84B26924C9C7F00ADB80AB6ED8ACEAE` (break `/Game/Blueprint/Structures/sStashSlot` (`|GetArrayItem` (`self.Stash`) (`|GetArrayItem` (`local.CompatibleSlots`))))))
                  (:`Is Valid`
                    (set `local.StrictTwoHanded?` (`|EnumEquality` (`/Game/Blueprint/Items/0_Item.WeaponHanded` _out_object) "NewEnumerator2"))))))
            (:`then_2`
              (if (not (`local.StrictTwoHanded?`))
                (goto _label)
                (else
                  ;[1 1 1] If the new item happens to be a strict 2 handed weapon, clear out all the slots then do the above
                  (for (_array_element_3 _array_index_2) (`local.CompatibleSlots`)
                    (set `local.Index` _array_element_3)
                    (switch `int` _array_index_2
                      (:`0`
                        (set `local.OldItem1` (`.Item_12_C84B26924C9C7F00ADB80AB6ED8ACEAE` (break `/Game/Blueprint/Structures/sStashSlot` _output)))
                        (bind _structout_3 (setmembers `/Game/Blueprint/Structures/sStashSlot` :`StructRef` _output :`Full?` false :`Item` null))
                        (`KismetArrayLibrary.Array_Set` (`self.Stash`) (`local.Index`) _structout_3))
                      (:`1`
                        (set `local.OldItem2` (`.Item_12_C84B26924C9C7F00ADB80AB6ED8ACEAE` (break `/Game/Blueprint/Structures/sStashSlot` _output_2)))
                        (bind _structout_4 (setmembers `/Game/Blueprint/Structures/sStashSlot` :`StructRef` _output_2 :`Full?` false :`Item` null))
                        (`KismetArrayLibrary.Array_Set` (`self.Stash`) (`local.Index`) _structout_4))))
                  (goto _label))))))))
    (:`then_3`
      ;[1 1 1] Refresh all touched slots, even if it has not been modified
      (for _array_element_4 (`local.CompatibleSlots`)
        (`self.RefreshStashSlot` _array_element_4))
      (`/Game/Blueprint/Items/0_Item.EquipItem` (`local.NewItem`) (`local.ItemIndex`))
      (return true (`local.OldItem1`) (`local.OldItem2`)))))