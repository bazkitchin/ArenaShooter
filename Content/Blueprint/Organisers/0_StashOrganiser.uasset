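; Stash organiser that manages the player's carried item slots and their equip and drop options.
; InitialiseStash builds the slot array and two-way links each slot to an ItemInInventory widget, refreshed as items change.
; AddItem fills the first free slot or reports overburden, while equipping returns up to two displaced items to the stash.
; SetOptions relabels options for Normal, Merchant or Stash contexts, though the bottom sell/store action is empty here.
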(event `TopOption`
  (params (Item :type "/Game/Blueprint/Items/0_Item Object Reference") (Index :type Integer))
  ;[1 1 1] Equip item and displace any item that was swapped (can be two with 2Handed Weapon)
  (bind (_accepted_ _displaceditem1 _displaceditem2) (`self.AddItem` (`/Game/Blueprint/MyGameInstance.Equipment` (`self.GameInstance`)) (`.Item_12_C84B26924C9C7F00ADB80AB6ED8ACEAE` (break `/Game/Blueprint/Structures/sStashSlot` (`|GetArrayItem` (`self.Stash`) Index))) Index))
  (if _accepted_
    (`|ExecutionSequence`
      (:`then_0`
        (`self.ClearIndex` Index))
      (:`then_1`
        (bind _out_object (`/Game/Blueprint/GeneralMacros.IsValidReturn` _displaceditem1)
          (:`Is Valid`
            (`/Game/Blueprint/Items/0_Item.UnequipItem` _out_object)
            (`self.AddItem` _out_object))))
      (:`then_2`
        (bind _out_object_2 (`/Game/Blueprint/GeneralMacros.IsValidReturn` _displaceditem2)
          (:`Is Valid`
            (`/Game/Blueprint/Items/0_Item.UnequipItem` _out_object_2)
            (`self.AddItem` _out_object_2))))
      (:`then_3`
        (`/Game/Blueprint/MyGameInstance.EquipmentHasChanged` (`self.GameInstance`))))))

(event `MiddleOption`
  (params (Index :type Integer))
  ;[1 1 1] Drop item
  (`/Game/Blueprint/Items/0_Item.ItemPutOnFloor` (`.Item_12_C84B26924C9C7F00ADB80AB6ED8ACEAE` (break `/Game/Blueprint/Structures/sStashSlot` (`|GetArrayItem` (`self.Stash`) Index))))
  (`self.ClearIndex` Index))

(event `BottomOption`
  (params (Index :type Integer)))

(fn `AddItem`
  (params (Item :type "/Game/Blueprint/Items/0_Item Object Reference") (SlotIndex :type Integer))
  (returns (`Accepted?` :type Boolean) (DisplacedItem1 :type "/Game/Blueprint/Items/0_Item Object Reference") (DisplacedItem2 :type "/Game/Blueprint/Items/0_Item Object Reference"))
  (locals (NewItem :type "/Game/Blueprint/Items/0_Item Object Reference"))
  (`|ExecutionSequence`
    (:`then_0`
      (bind _output_get (set `local.NewItem` Item))
      (`/Game/Blueprint/GeneralMacros.IsValidReturn` _output_get
        (:`Is Not Valid`
          (return false null null))))
    (:`then_1`
      (for (_array_element _array_index) (`self.Stash`)
        (if (not (`.Full?_11_AC9CC015470371E7BC599091DAFEB896` (break `/Game/Blueprint/Structures/sStashSlot` _array_element)))
          (bind _structout (setmembers `/Game/Blueprint/Structures/sStashSlot` :`StructRef` _array_element :`Full?` true :`Item` (`local.NewItem`)))
          (`KismetArrayLibrary.Array_Set` (`self.Stash`) _array_index _structout)
          (`self.RefreshStashSlot` _array_index)
          (return true null null)))
      (`/Game/Blueprint/MyGameInstance.PlayerIsOverBurdened` (`self.GameInstance`) (`local.NewItem`))
      (return false null null))))

(fn `ClearIndex`
  (params (Index :type Integer))
  (bind (_index _full_ _item _linkeditemininventory _alloweditems) (break `/Game/Blueprint/Structures/sStashSlot` (`|GetArrayItem` (`self.Stash`) Index)))
  ;[1 1 1] Clears the 'Full' flag and the Updates of the linked UMG
  (bind _out_object (`/Game/Blueprint/GeneralMacros.IsValidReturn` _linkeditemininventory)
    (:`Is Valid`
      (`/Game/UMG/ItemInInventory.UpdateSlot` _out_object false null))
    (:`Is Not Valid`
      _))
  (`KismetArrayLibrary.Array_Set` (`self.Stash`) Index (make `/Game/Blueprint/Structures/sStashSlot` _index false null _linkeditemininventory _alloweditems)))

(fn `InitialiseStash`
  (params (NumberOfSlots :type Integer) (ListOfItemInInventory :type "Array of /Game/UMG/ItemInInventory Object Reference"))
  (`|ExecutionSequence`
    (:`then_0`
      (set `self.NumberOfSlots` NumberOfSlots))
    (:`then_1`
      ;[1 1 1] If the stash is not organised, i.e externally defined; create all the slots
      (for _index (range (+ (`/Game/Blueprint/GeneralMacros.Minus1` (`self.NumberOfSlots`)) 1))
        (`KismetArrayLibrary.Array_Add` (`self.Stash`) (make `/Game/Blueprint/Structures/sStashSlot` _index))))
    (:`then_2`
      (if (== (`self.NumberOfSlots`) (`KismetArrayLibrary.Array_Length` ListOfItemInInventory))
        ;[1 1 1] If the stash has a matching UMG array link them up
        (for (_array_element _array_index) ListOfItemInInventory
          (`self.LinkStashSlotToItemInventory` _array_element _array_index))
        (else
          (`KismetSystemLibrary.PrintString` null "StashOrganiser not set up correctly"))))))

(fn `LinkStashSlotToItemInventory`
  (params (ItemInInventory :type "/Game/UMG/ItemInInventory Object Reference") (SlotNumber :type Integer))
  (returns (Success :type Boolean))
  (locals (LocalSuccess :type Boolean :default true) (LocalIndex :type Integer))
  (set `local.LocalIndex` SlotNumber)
  (if (`KismetArrayLibrary.Array_IsValidIndex` (`self.Stash`) (`local.LocalIndex`))
    ;[1 1 1] Link the stash index with its ItemInInventory UMG, so they can be automatically maintained
    (bind _structout (setmembers `/Game/Blueprint/Structures/sStashSlot` :`StructRef` (`|GetArrayItem` (`self.Stash`) (`local.LocalIndex`)) :`LinkedItemInInventory` ItemInInventory))
    (`KismetArrayLibrary.Array_Set` (`self.Stash`) (`local.LocalIndex`) _structout)
    ;[1 1 1] Link, if possible, the ItemInInventory back to this Stash Organiser, so it can be used for feedback; such as option selections
    (bind _out_object (`/Game/Blueprint/GeneralMacros.IsValidReturn` (`.LinkedItemInInventory_16_B26310CC4AF33163DF838F9EC335AF87` (break `/Game/Blueprint/Structures/sStashSlot` (`|GetArrayItem` (`self.Stash`) (`local.LocalIndex`)))))
      (:`Is Valid`
        (`/Game/UMG/ItemInInventory.LinkToStashOrganiser` _out_object self (`local.LocalIndex`))
        (`self.RefreshStashSlot` (`local.LocalIndex`)))
      (:`Is Not Valid`
        _))
    (return (`local.LocalSuccess`))
    (else
      ;[1 1 1] If it wasn't return false
      (bind _output_get (set `local.LocalSuccess` false))
      (return _output_get))))

(fn `RefreshStashSlot`
  (params (Index :type Integer))
  (bind ((`Full?_11_AC9CC015470371E7BC599091DAFEB896` _full_) (`Item_12_C84B26924C9C7F00ADB80AB6ED8ACEAE` _item) (`LinkedItemInInventory_16_B26310CC4AF33163DF838F9EC335AF87` _linkeditemininventory)) (break `/Game/Blueprint/Structures/sStashSlot` (`|GetArrayItem` (`self.Stash`) Index)))
  (bind _out_object (`/Game/Blueprint/GeneralMacros.IsValidReturn` _linkeditemininventory)
    (:`Is Valid`
      (`/Game/UMG/ItemInInventory.UpdateSlot` _out_object _full_ _item))))

(fn `SetOptions`
  (params (Environment :type "/Game/Blueprint/Enumerations/eTypesOfStash Enum" :default "NewEnumerator0"))
  (switch `/Game/Blueprint/Enumerations/eTypesOfStash` Environment
    (:`NewEnumerator0`
      (`self.SetOptionText` "Equip Item" "Drop Item" "Not Available" true true))
    (:`NewEnumerator2`
      (`self.SetOptionText` "Equip Item" "Drop Item" "Sell Item" true true true))
    (:`NewEnumerator3`
      (`self.SetOptionText` "Equip Item" "Drop Item" "Store Item" true true true))))

(fn `SetOptionText`
  (params (Top :type Text) (Middle :type Text) (Bottom :type Text) (EnableTop :type Boolean) (EnableMiddle :type Boolean) (EnableBottom :type Boolean))
  (`|ExecutionSequence`
    (:`then_0`
      (set `self.TopOptionText` Top))
    (:`then_1`
      (set `self.MiddleOptionText` Middle))
    (:`then_2`
      (set `self.BottomOptionText` Bottom))
    (:`then_3`
      (set `self.EnableTopOption` EnableTop))
    (:`then_4`
      (set `self.EnableMiddleOption` EnableMiddle))
    (:`then_5`
      (set `self.EnableBottomOption` EnableBottom))))