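; Targeted attack actor that calls in a Stormtalon over its location and spins a top location marker every tick.
; On BeginPlay it tries random entry and exit points on an elevated ring, using visibility traces to find clear paths from above the target.
; It then spawns the Stormtalon with the route, ground target and Benefactor as owning vehicle, using the last points tried if none pass.
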(event `PassPlausibiltyCheck`
  (bind _returnvalue (`KismetMathLibrary.MakeVector` (`self.SpawnDistance`)))
  (bind _returnvalue_2 (+ (`self.K2_GetActorLocation`) (`KismetMathLibrary.MakeVector` 0.0 0.0 (`self.SpawnHeight`))))
  (bind _returnvalue_3 (+ (`self.K2_GetActorLocation`) (`KismetMathLibrary.MakeVector` 0.0 0.0 (`self.SpawnHeight`))))
  (goto _label :!via `Break`))

(event `self.ReceiveBeginPlay`
  (bind _returnvalue (`self.K2_GetActorLocation`))
  (bind _spawnlocation (`self.SpawnLocation`))
  (bind _returnvalue_2 (`KismetMathLibrary.MakeVector` (`self.SpawnDistance`)))
  (bind _returnvalue_3 (+ (`self.K2_GetActorLocation`) (`KismetMathLibrary.MakeVector` 0.0 0.0 (`self.SpawnHeight`))))
  (bind _returnvalue_4 (+ (`self.K2_GetActorLocation`) (`KismetMathLibrary.MakeVector` 0.0 0.0 (`self.SpawnHeight`))))
  (`|ExecutionSequence`
    (:`then_0`
      (for _ (range 51) :!label _label
        (set `self.ExitLocation` (+ _returnvalue_3 (`KismetMathLibrary.GreaterGreater_VectorRotator` _returnvalue_2 (`KismetMathLibrary.MakeRotator` 0.0 0.0 (`KismetMathLibrary.RandomFloatInRange` 0.0 360.0)))))
        (set `self.SpawnLocation` (+ _returnvalue_3 (`KismetMathLibrary.GreaterGreater_VectorRotator` _returnvalue_2 (`KismetMathLibrary.MakeRotator` 0.0 0.0 (`KismetMathLibrary.RandomFloatInRange` 0.0 360.0)))))
        (bind (_outhit _returnvalue_5) (`KismetSystemLibrary.LineTraceSingle` _returnvalue_4 (`self.SpawnLocation`) "TraceTypeQuery1"))
        (bind (_outhit_2 _returnvalue_6) (`KismetSystemLibrary.LineTraceSingle` _returnvalue_4 (`self.ExitLocation`) "TraceTypeQuery1"))
        (if (not (or _returnvalue_5 _returnvalue_6))
          (`self.PassPlausibiltyCheck`))))
    (:`then_1`
      (bind _returnvalue_7 (`|SpawnActorFromClass` "/Game/Blueprint/Characters/StormTalon/1_Stormtalon.1_Stormtalon_C" (`KismetMathLibrary.MakeTransform` _spawnlocation) "Undefined" "OverrideRootScale" self (+ _returnvalue (`KismetMathLibrary.MakeVector` 0.0 0.0 (`self.SpawnHeight`))) _spawnlocation (`self.ExitLocation`) _returnvalue (`self.Benefactor`) null))
      (set `self.MyStormtalon` _returnvalue_7))))

(event `self.ReceiveTick`
  (params (DeltaSeconds :type "Float (single-precision)"))
  (`SceneComponent.K2_AddLocalRotation` (`self.LocationMarkerTop`) (`KismetMathLibrary.MakeRotator` 0.0 0.0 (* DeltaSeconds 180.0)) false false))

(fn `UserConstructionScript`)