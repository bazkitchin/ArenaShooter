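; Base shooter pawn shared by human and AI players, handling gun fire, health, kill/death counts and respawning.
; Tick pitches the gun with control rotation and, for InGameController players, updates HUD health and bobs the gun.
; ShotGun fires cooldown-gated line traces, randomly offset for AI, damaging iInteractive actors; repeated misses make AI drop targets.
; Lethal damage credits the killer and respawns via InGameMode; construction randomises body colour, reused by death particles.
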(event `self.ReceiveBeginPlay`
  (set `self.StatingGunOffset` (`SceneComponent.GetRelativeTransform` (`self.Gun`))))

(event `self.ReceiveTick`
  (params (DeltaSeconds :type "Float (single-precision)"))
  (bind _returnvalue (`self.K2_GetActorLocation`))
  (`|ExecutionSequence`
    (:`then_0`
      (bind _output_get (set `self.GunCooldown` (+ DeltaSeconds (`self.GunCooldown`))))
      (bind _asin_game_controller (cast `/Game/Blueprint/InGameController` (`self.GetController`)))
      (`/Game/UMG/HUD.UpdateHealth` (`/Game/Blueprint/InGameController.HUD` _asin_game_controller) (`self.CurrentHealth`))
      (if (not (== (`self.PreviousLocation`) _returnvalue))
        (bind _output_get_2 (set `self.GunBob` (+ (`self.GunBob`) 7.5)))
        (bind _returnvalue_2 (* (`KismetMathLibrary.DegSin` _output_get_2) -1.0))
        (`SceneComponent.K2_AddLocalOffset` (`self.Gun`) (`KismetMathLibrary.MakeVector` _returnvalue_2 0.0 _returnvalue_2) false false)
        (else
          (set `self.GunBob` 0.0)
          (`SceneComponent.K2_SetRelativeLocation` (`self.Gun`) (.location (`self.StatingGunOffset`)) false false)))
      (set `self.PreviousLocation` _returnvalue))
    (:`then_1`
      (`SceneComponent.K2_SetRelativeRotation` (`self.Gun`) (`KismetMathLibrary.MakeRotator` 0.0 (+ (.pitch (`self.GetControlRotation`)) 90.0)) false false))))

(event `ShotGun`
  (bind _barrel (`self.Barrel`))
  (bind _returnvalue (`SceneComponent.K2_GetComponentLocation` _barrel))
  (if (> (`self.GunCooldown`) (`self.GunFireRate`))
    (set `self.GunCooldown` 0.0)
    (bind _adjustmentvector (`self.AdjustShotForDifficulty` (`self.GetController`)))
    (bind _returnvalue_2 (+ _adjustmentvector _returnvalue (`KismetMathLibrary.GreaterGreater_VectorRotator` (1000.0 0.0 0.0) (`SceneComponent.K2_GetComponentRotation` _barrel))))
    (`GameplayStatics.SpawnEmitterAtLocation` "/Game/ParticleSystems/P_Bullet.P_Bullet" _returnvalue (`KismetMathLibrary.FindLookAtRotation` _returnvalue _returnvalue_2))
    (bind (_outhit _returnvalue_3) (`KismetSystemLibrary.LineTraceSingle` _returnvalue _returnvalue_2 "TraceTypeQuery1"))
    (if _returnvalue_3
      (bind (_bblockinghit _binitialoverlap _time _distance _location _impactpoint _normal _impactnormal _physmat _hitactor) (`GameplayStatics.BreakHitResult` _outhit))
      (`GameplayStatics.SpawnEmitterAtLocation` "/Game/ParticleSystems/P_BulletImpact.P_BulletImpact" _location (`KismetMathLibrary.Conv_VectorToRotator` _normal))
      (bind (_asi_interactive _bsuccess) (cast `/Game/Blueprint/iInteractive` _hitactor :!pure true))
      (if _bsuccess
        (set `self.TimesMissed` 0)
        (`/Game/Blueprint/iInteractive.AffectHealth` _asi_interactive (`self.GunDamage`) self)
        (elif (> (`self.TimesMissed`) 5)
          (`self.TargetLost`)
          (set `self.TimesMissed` 0)
          (else
            (`/Engine/EditorBlueprintResources/StandardMacros.IncrementInt` (`self.TimesMissed`))))))))

(event `/Game/Blueprint/iInteractive.AffectHealth`
  (params (Amount :type Integer) (SourceActor :type "Actor Object Reference"))
  (`AudioComponent.Play` (`self.GunShot`) 0.0)
  (bind _output_get (set `self.CurrentHealth` (- (`self.CurrentHealth`) Amount)))
  (if (<= _output_get 0)
    (`|ExecutionSequence`
      (:`then_0`
        (bind _as0_base_player (cast `/Game/Blueprint/0_BasePlayer` SourceActor))
        (`self.TargetLost` _as0_base_player)
        (`self.KillEnemy` _as0_base_player))
      (:`then_2`
        (`self.Died`)))))

(event `Died`
  (bind (_r _g _b) (break `LinearColor` (`self.PlayerColour`)))
  (bind _returnvalue (`GameplayStatics.SpawnEmitterAtLocation` "/Game/ParticleSystems/P_CubeDeath.P_CubeDeath" (`self.K2_GetActorLocation`)))
  (`ParticleSystemComponent.SetVectorParameter` _returnvalue "PlayerColour" (`KismetMathLibrary.MakeVector` _r _g _b))
  (set `self.Deaths` (+ (`self.Deaths`) 1))
  (`self.TargetLost`)
  (bind _spawnpoint (`/Game/Blueprint/InGameMode.GetSpawnLocation` (cast `/Game/Blueprint/InGameMode` (`GameplayStatics.GetGameMode`) :!pure true)))
  (`self.K2_SetActorTransform` _spawnpoint false true)
  (set `self.CurrentHealth` (`self.StartingHealth`)))

(event `TargetLost`
  (bind _asai_basic (cast `/Game/AI/AI_Basic` (`self.GetController`)))
  (`/Game/AI/AI_Basic.PawnDied` _asai_basic))

(event `KillEnemy`
  (set `self.Kills` (+ (`self.Kills`) 1)))

(fn `AdjustShotForDifficulty`
  (params (Controller :type "Controller Object Reference"))
  (returns (AdjustmentVector :type "Vector Structure"))
  (locals (AIControlled :type Boolean) (Inaccurary :type "Vector Structure" :default (0.0 0.0 0.0)))
  (cast `AIController` Controller
    (:`then`
      (set `local.AIControlled` true)
      (bind _output_get (set `local.Inaccurary` (`KismetMathLibrary.MakeVector` 0.0 (`KismetMathLibrary.RandomFloatInRange` -500.0 500.0) (`KismetMathLibrary.RandomFloatInRange` -500.0 500.0))))
      (set `local.Inaccurary` _output_get))
    (:`CastFailed`
      (set `local.AIControlled` false)
      (set `local.Inaccurary` (0.0 0.0 0.0))))
  (return (`local.Inaccurary`)))

(fn `UserConstructionScript`
  (bind _returnvalue (`PrimitiveComponent.CreateDynamicMaterialInstance` (`self.Body`) 0 "/Game/Materials/Mat_Plastic.Mat_Plastic"))
  (bind _output_get (set `self.PlayerColour` (make `LinearColor` (`KismetMathLibrary.RandomFloat`) 0.2 (`KismetMathLibrary.RandomFloat`) 1.0)))
  (`MaterialInstanceDynamic.SetVectorParameterValue` _returnvalue "Base Color" _output_get)
  (bind _returnvalue_2 (`PrimitiveComponent.CreateDynamicMaterialInstance` (`self.Gun`) 0 "/Game/Materials/Mat_Plasma.Mat_Plasma"))
  (bind _output_get_2 (set `self.GunColor` _returnvalue_2))
  (`MaterialInstanceDynamic.SetScalarParameterValue` _output_get_2 "EmissionMulti" 0.0))