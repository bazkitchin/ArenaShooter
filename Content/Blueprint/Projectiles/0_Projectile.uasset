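; Base projectile Blueprint that counts down TimeRemaining on Tick and calls TimedOut, which destroys it.
; SphereTraceAtLocation finds hits in a radius, line-traces to each impact point, and passes the first blocking actor to ForEachInteractiveHit if it casts to iInteractive.
; ForEachInteractiveHit is an empty hook, and nothing here calls the trace.
; A helper spawns an optional particle effect and sound at the projectile's location.
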(event `self.ReceiveBeginPlay`)

(event `self.ReceiveTick`
  (params (DeltaSeconds :type "Float (single-precision)"))
  (bind _output_get (set `self.TimeRemaining` (- (`self.TimeRemaining`) (`GameplayStatics.GetWorldDeltaSeconds`))))
  (if (<= _output_get 0.0)
    (`self.TimedOut`)))

(event `TimedOut`
  (`self.K2_DestroyActor`))

(event `SphereTraceAtLocation`
  (params (Radius :type "Float (double-precision)") (Debug :type Boolean))
  (bind _returnvalue (`self.K2_GetActorLocation`))
  (bind _outhits (`KismetSystemLibrary.SphereTraceMulti` :`Start` _returnvalue :`End` _returnvalue :`Radius` Radius :`TraceChannel` "TraceTypeQuery1" :`DrawDebugType` (select `bool` Debug :`true` "ForDuration" :!type "EDrawDebugTrace Enum")))
  (for _array_element _outhits
    (bind _outhit (`KismetSystemLibrary.LineTraceSingle` (`self.K2_GetActorLocation`) (`.ImpactPoint` (`GameplayStatics.BreakHitResult` _array_element)) "TraceTypeQuery1"))
    (bind _asi_interactive (cast `/Game/Blueprint/Interfaces/iInteractive` (`.HitActor` (`GameplayStatics.BreakHitResult` _outhit))))
    (`self.ForEachInteractiveHit` _asi_interactive)))

(event `ForEachInteractiveHit`
  (params (iInteractive :type "/Game/Blueprint/Interfaces/iInteractive Interface")))

(fn `SpawnParticleSoundAtLocation`
  (params (EmitterTemplate :type "ParticleSystem Object Reference") (Sound :type "SoundBase Object Reference"))
  (bind _returnvalue (`self.K2_GetActorLocation`))
  (`|ExecutionSequence`
    (:`then_0`
      (`/Engine/EditorBlueprintResources/StandardMacros.IsValid` EmitterTemplate
        (:`Is Valid`
          (`GameplayStatics.SpawnEmitterAtLocation` EmitterTemplate _returnvalue))))
    (:`then_1`
      (`/Engine/EditorBlueprintResources/StandardMacros.IsValid` Sound
        (:`Is Valid`
          (`GameplayStatics.SpawnSoundAtLocation` Sound _returnvalue))))))

(fn `UserConstructionScript`)