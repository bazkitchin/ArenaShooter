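; Grenade projectile that bounces and explodes when its timer runs out, damaging interactive objects nearby.
; An initial velocity impulse on the mesh launches it at BeginPlay, and sufficiently hard hits play a metal bounce sound after a short delay.
; On TimedOut it spawns explosion effects and runs a sphere trace before calling the parent.
; ForEachInteractiveHit damages targets through AffectHealth on the IInteractive interface, crediting the Benefactor.
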(event `self.ReceiveBeginPlay`
  (`parent.ReceiveBeginPlay`)
  (`PrimitiveComponent.AddImpulse` (`self.Mesh`) (`self.InitialImpulse`) "None" true))

(event `self.ReceiveTick`
  (params (DeltaSeconds :type "Float (single-precision)"))
  (`parent.ReceiveTick` DeltaSeconds))

(event `self.TimedOut`
  (`self.SpawnParticleSoundAtLocation` "/Game/StarterContent/Particles/P_Explosion.P_Explosion" "/Game/StarterContent/Audio/Explosion01.Explosion01")
  (`self.SphereTraceAtLocation` 500.0)
  (`parent.TimedOut`))

(event `self.ForEachInteractiveHit`
  (params (iInteractive :type "/Game/Blueprint/Interfaces/iInteractive Interface"))
  (`/Game/Blueprint/Interfaces/iInteractive.AffectHealth` iInteractive 100 (`self.Benefactor`)))

(event `self.Mesh.OnComponentHit`
  (params (HitComponent :type "PrimitiveComponent Object Reference") (OtherActor :type "Actor Object Reference") (OtherComp :type "PrimitiveComponent Object Reference") (NormalImpulse :type "Vector Structure") (Hit :type "HitResult Structure (by ref)"))
  (if (> (`KismetMathLibrary.VSize` NormalImpulse) 90.0)
    (`KismetSystemLibrary.Delay` 0.1)
    (`GameplayStatics.SpawnSoundAtLocation` "/Game/Audio/MetalBounce.MetalBounce" (`self.K2_GetActorLocation`))))

(fn `UserConstructionScript`
  (`parent.UserConstructionScript`))