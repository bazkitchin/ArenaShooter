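; Rocket projectile that flies forward and explodes on a blocking hit or timeout, dealing area damage to players.
; Tick moves it by swept offsets and, once the lock timer expires, lerps its rotation toward a fixed target location until aligned, then stops steering.
; Detonation runs once, spawning effects and a sphere trace that skips the firing player's teammates, then destroys the actor after a delay for the trail.
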(event `self.ReceiveTick`
  (params (DeltaSeconds :type "Float (single-precision)"))
  (bind _returnvalue (`self.K2_GetActorRotation`))
  (bind _returnvalue_2 (`KismetMathLibrary.FindLookAtRotation` (`self.K2_GetActorLocation`) (`self.TargetLocation`)))
  (`parent.ReceiveTick` DeltaSeconds)
  (bind _output_get (set `self.TargetLockTime` (- (`self.TargetLockTime`) (`GameplayStatics.GetWorldDeltaSeconds`))))
  (if (or (> _output_get 0.0) (`self.DisableTargetLock`))
    _
    (elif (== _returnvalue _returnvalue_2 :`ErrorTolerance` 0.5)
      (set `self.DisableTargetLock` true)
      (else
        (`self.K2_SetActorRotation` (`KismetMathLibrary.RLerp` _returnvalue _returnvalue_2 0.25 true)))))
  (bind _sweephitresult (`self.K2_AddActorWorldOffset` (`KismetMathLibrary.GreaterGreater_VectorRotator` (`KismetMathLibrary.MakeVector` (* (`self.Speed`) (`GameplayStatics.GetWorldDeltaSeconds`))) (`self.K2_GetActorRotation`)) true))
  (bind (_bblockinghit _binitialoverlap) (`GameplayStatics.BreakHitResult` _sweephitresult))
  (if (or _bblockinghit _binitialoverlap)
    (`self.TimedOut`)))

(event `self.ReceiveHit`
  (params (MyComp :type "PrimitiveComponent Object Reference") (Other :type "Actor Object Reference") (OtherComp :type "PrimitiveComponent Object Reference") (bSelfMoved :type Boolean) (HitLocation :type "Vector Structure") (HitNormal :type "Vector Structure") (NormalImpulse :type "Vector Structure") (Hit :type "HitResult Structure (by ref)"))
  (`self.TimedOut`))

(event `self.TimedOut`
  (bind _mesh (`self.Mesh`))
  (if (not (`self.Exploded`))
    (set `self.Exploded` true)
    (`self.SpawnParticleSoundAtLocation` "/Game/StarterContent/Particles/P_Explosion.P_Explosion" "/Game/StarterContent/Audio/Explosion02.Explosion02")
    (`self.SphereTraceAtLocation` 500.0)
    (`SceneComponent.SetHiddenInGame` _mesh true false)
    (`PrimitiveComponent.SetCollisionEnabled` _mesh "NoCollision")
    (`ActorComponent.SetActive` (`self.RocketSound`) false false)
    (`ActorComponent.Deactivate` (`self.RocketTrail`))
    (set `self.Speed` 0.0)
    (`KismetSystemLibrary.Delay` 2.0)
    (`self.K2_DestroyActor`)))

(event `self.ForEachInteractiveHit`
  (params (iInteractive :type "/Game/Blueprint/Interfaces/iInteractive Interface"))
  (bind _as0_base_player (cast `/Game/Blueprint/Characters/0_BasePlayer` iInteractive))
  (bind _as0_base_player_2 (cast `/Game/Blueprint/Characters/0_BasePlayer` (`self.Benefactor`))
    (:`then`
      (if (not (== (`/Game/Blueprint/Characters/0_BasePlayer.Team` _as0_base_player) (`/Game/Blueprint/Characters/0_BasePlayer.Team` _as0_base_player_2)))
        (`/Game/Blueprint/Interfaces/iInteractive.AffectHealth` iInteractive 100 (`self.Benefactor`) :!label _label)))
    (:`CastFailed`
      (goto _label))))

(fn `UserConstructionScript`
  (`parent.UserConstructionScript`))