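; Base-style pickup prop that stands in for a hidden item actor until the player collects it.
; A radius-configurable overlap sphere shows and removes a prompt widget, updated on Tick, as the player enters and leaves.
; LookingAt calls set a flag that Tick consumes each frame to toggle a custom depth stencil highlight.
; PickupObject gives the item to the player, unhides it, clears the prompt and destroys the pickup.
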(event `self.ReceiveBeginPlay`
  (`/Engine/EditorBlueprintResources/StandardMacros.IsValid` (`self.ActualItem`)
    (:`Is Valid`
      (`self.K2_SetActorTransform` (`self.ActualItem`) (`self.GetTransform`) false true)
      (`self.SetActorHiddenInGame` (`self.ActualItem`) true))))

(event `self.ReceiveTick`
  (params (DeltaSeconds :type "Float (single-precision)"))
  (bind _pickuptext (`self.PickupText`))
  (if (`self.PlayerLookingAt`)
    (`self.AddHighlight`)
    (set `self.PlayerLookingAt` false)
    (else
      (`self.RemoveHighlight`)))
  (`/Engine/EditorBlueprintResources/StandardMacros.IsValid` _pickuptext
    (:`Is Valid`
      (`/Game/UMG/PickText.Update` _pickuptext))))

(event `self.PickupArea.OnComponentBeginOverlap`
  (params (OverlappedComponent :type "PrimitiveComponent Object Reference") (OtherActor :type "Actor Object Reference") (OtherComp :type "PrimitiveComponent Object Reference") (OtherBodyIndex :type Integer) (bFromSweep :type Boolean) (SweepResult :type "HitResult Structure (by ref)"))
  (`/Engine/EditorBlueprintResources/StandardMacros.IsValid` (`self.PickupText`)
    (:`Is Not Valid`
      (cast `/Game/Blueprint/Characters/1_PlayerBase` OtherActor)
      (bind _returnvalue (`|CreateWidget` "/Game/UMG/PickText.PickText_C" (`GameplayStatics.GetPlayerController` 0) self))
      (bind _output_get (set `self.PickupText` _returnvalue))
      (`UserWidget.AddToViewport` _output_get 0))))

(event `self.PickupArea.OnComponentEndOverlap`
  (params (OverlappedComponent :type "PrimitiveComponent Object Reference") (OtherActor :type "Actor Object Reference") (OtherComp :type "PrimitiveComponent Object Reference") (OtherBodyIndex :type Integer))
  (bind _pickuptext (`self.PickupText`))
  (`/Engine/EditorBlueprintResources/StandardMacros.IsValid` (`self.PickupText`) :!label _label
    (:`Is Valid`
      (cast `/Game/Blueprint/Characters/1_PlayerBase` OtherActor)
      (`Widget.RemoveFromParent` _pickuptext)
      (`/Game/UMG/PickText.Destroy` _pickuptext)
      (set `self.PickupText` null))))

(event `PickedUp`
  (goto _label))

(event `LookingAt`
  (set `self.PlayerLookingAt` true))

(event `PickupObject`
  (params (`WhomIsPickMeUp?` :type "Actor Object Reference"))
  (bind _actualitem (`self.ActualItem`))
  (bind _as1_player_base (cast `/Game/Blueprint/Characters/1_PlayerBase` `WhomIsPickMeUp?`))
  (`/Game/Blueprint/Characters/1_PlayerBase.GivePlayerItem` _as1_player_base _actualitem)
  (`self.SetActorHiddenInGame` _actualitem false)
  (`KismetSystemLibrary.PrintString` (`KismetStringLibrary.Concat_StrStr` "Player picked up " (`self.Name`)))
  (set `self.PlayerLookingAt` false)
  (`self.PickedUp`)
  (`self.K2_DestroyActor`))

(fn `AddHighlight`
  (bind _pickupmesh (`self.PickUpMesh`))
  (`PrimitiveComponent.SetRenderCustomDepth` _pickupmesh true)
  (`PrimitiveComponent.SetCustomDepthStencilValue` _pickupmesh 1))

(fn `RemoveHighlight`
  (`PrimitiveComponent.SetRenderCustomDepth` (`self.PickUpMesh`) false))

(fn `UserConstructionScript`
  (`SphereComponent.SetSphereRadius` (`self.PickupArea`) (`self.PickupRadius`) true))