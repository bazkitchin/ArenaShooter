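; Game instance that holds the player's character list, 40-slot item stash and equipped gear.
; Init builds the stash grid and loads the character-name list from a save slot, saving one if loading fails.
; AddItemToEquipment swaps gear by type, with special trinket and weapon-handedness rules, returning replaced items; stash and equipment changes push to HUD inventory slots.
; A macro iterates valid equipment; LoadCharacter, DropPlayerItem and RefreshStash are empty stubs.
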(event `self.ReceiveInit`
  (`|ExecutionSequence`
    (:`then_0`
      (`self.InitialiseStash`))
    (:`then_1`
      (bind _success (`self.LoadCharacterList`))
      (if _success
        (`KismetSystemLibrary.PrintString` "Init: Loaded character list" true true (struct :`G` 1.0 :`A` 1.0))
        (else
          (`KismetSystemLibrary.PrintString` "Init: Failed! Loading character list" true true (struct :`R` 1.0 :`A` 1.0) 4.0)
          (`self.SaveCharacterList`))))))

(event `LoadCharacter`
  (params (CharacterName :type String)))

(event `GivePlayerItem`
  (params (Item :type "/Game/Blueprint/Items/0_Item Object Reference"))
  (`self.AddItemToStash` Item))

(event `DropPlayerItem`)

(fn `AddItemToEquipment`
  (params (Item :type "/Game/Blueprint/Items/0_Item Object Reference"))
  (returns (ReplacedEquipment :type "/Game/Blueprint/Items/0_Item Object Reference") (OtherReplacedEquipment :type "/Game/Blueprint/Items/0_Item Object Reference"))
  (locals (NewItem :type "/Game/Blueprint/Items/0_Item Object Reference") (OldItem :type "/Game/Blueprint/Items/0_Item Object Reference") (OtherOldItem :type "/Game/Blueprint/Items/0_Item Object Reference") (OrigLeftWeapon :type "/Game/Blueprint/Items/0_Item Object Reference") (OrigRightWeapon :type "/Game/Blueprint/Items/0_Item Object Reference"))
  (bind _origrightweapon (`local.OrigRightWeapon`))
  (bind _origrightweapon_2 (`local.OrigRightWeapon`))
  (bind (_helmet _shoulders _chest _backpack _arms _belt _legs _lefthandweapon _righthandweapon) (break `/Game/Blueprint/Structures/sCharacterEquipment` (`self.Equipment`)))
  (bind (_helmet_2 _shoulders_2 _chest_2 _backpack_2 _arms_2 _belt_2 _legs_2) (break `/Game/Blueprint/Structures/sCharacterEquipment` (`self.Equipment`)))
  (bind (_helmet_3 _shoulders_3 _chest_3 _backpack_3 _arms_3 _belt_3 _legs_3 _lefthandweapon_2 _righthandweapon_2 _trinket1 _trinket2) (break `/Game/Blueprint/Structures/sCharacterEquipment` (`self.Equipment`)))
  (bind _asmy_game_instance (cast `/Game/Blueprint/MyGameInstance` (`GameplayStatics.GetGameInstance`) :!pure true))
  (bind _asmy_game_instance_2 (cast `/Game/Blueprint/MyGameInstance` (`GameplayStatics.GetGameInstance`) :!pure true))
  (bind _inventorypanel (`/Game/UMG/HUD.InventoryPanel` (`/Game/Blueprint/InGameController.HUD` (cast `/Game/Blueprint/InGameController` (`GameplayStatics.GetPlayerController` 0) :!pure true))))
  (bind _inventorypanel_2 (`/Game/UMG/HUD.InventoryPanel` (`/Game/Blueprint/InGameController.HUD` (cast `/Game/Blueprint/InGameController` (`GameplayStatics.GetPlayerController` 0) :!pure true))))
  (bind _inventorypanel_3 (`/Game/UMG/HUD.InventoryPanel` (`/Game/Blueprint/InGameController.HUD` (cast `/Game/Blueprint/InGameController` (`GameplayStatics.GetPlayerController` 0) :!pure true))))
  (bind _inventorypanel_4 (`/Game/UMG/HUD.InventoryPanel` (`/Game/Blueprint/InGameController.HUD` (cast `/Game/Blueprint/InGameController` (`GameplayStatics.GetPlayerController` 0) :!pure true))))
  (bind _lefthand (`/Game/UMG/InventoryPanel.LeftHand` _inventorypanel_2))
  (bind _righthand (`/Game/UMG/InventoryPanel.RightHand` _inventorypanel_4))
  (bind _lefthand_2 (`/Game/UMG/InventoryPanel.LeftHand` _inventorypanel_4))
  (`|ExecutionSequence`
    (:`then_0`
      (bind _output_get (set `local.NewItem` Item))
      (switch `/Game/Blueprint/Enumerations/eItemTYpes` (`/Game/Blueprint/Items/0_Item.Type` _output_get)
        (:`NewEnumerator0`
          ;[1 1 1] Normal items are straight replacements for old ones
          (`self.UpdateEquimentSlot` _helmet_2 "NewEnumerator0" (`/Game/UMG/InventoryPanel.Helmet` _inventorypanel_3) (`local.NewItem`)))
        (:`NewEnumerator1`
          (`self.UpdateEquimentSlot` _shoulders_2 "NewEnumerator1" (`/Game/UMG/InventoryPanel.Shoulders` _inventorypanel_3) (`local.NewItem`)))
        (:`NewEnumerator2`
          (`self.UpdateEquimentSlot` _chest_2 "NewEnumerator2" (`/Game/UMG/InventoryPanel.Chest` _inventorypanel_3) (`local.NewItem`)))
        (:`NewEnumerator3`
          (`self.UpdateEquimentSlot` _backpack_2 "NewEnumerator3" (`/Game/UMG/InventoryPanel.Backpack` _inventorypanel_3) (`local.NewItem`)))
        (:`NewEnumerator4`
          (`self.UpdateEquimentSlot` _arms_2 "NewEnumerator4" (`/Game/UMG/InventoryPanel.Arms` _inventorypanel_3) (`local.NewItem`)))
        (:`NewEnumerator5`
          (`self.UpdateEquimentSlot` _belt_2 "NewEnumerator5" (`/Game/UMG/InventoryPanel.Belt` _inventorypanel_3) (`local.NewItem`)))
        (:`NewEnumerator6`
          (`self.UpdateEquimentSlot` _legs_2 "NewEnumerator6" (`/Game/UMG/InventoryPanel.Legs` _inventorypanel_3) (`local.NewItem`)))
        (:`NewEnumerator7`
          ;[1 1 1] Deal with swapping trinkets, fill left then right, if they are both full swap the left
          (`/Engine/EditorBlueprintResources/StandardMacros.IsValid` _trinket1
            (:`Is Valid`
              (`/Engine/EditorBlueprintResources/StandardMacros.IsValid` _trinket2
                (:`Is Valid`
                  (set `local.OldItem` _trinket1)
                  (`self.SetEquipmentSlot` _asmy_game_instance_2 "NewEnumerator10" (`local.NewItem`) :!label _label)
                  (`/Game/UMG/ItemInInventory.UpdateSlot` (`/Game/UMG/InventoryPanel.TrinketRight` _inventorypanel) true (`local.NewItem`)))
                (:`Is Not Valid`
                  (set `local.OldItem` null)
                  (`self.SetEquipmentSlot` _asmy_game_instance_2 "NewEnumerator9" (`local.NewItem`))
                  (`/Game/UMG/ItemInInventory.UpdateSlot` (`/Game/UMG/InventoryPanel.TrinketLeft` _inventorypanel) true (`local.NewItem`)))))
            (:`Is Not Valid`
              (set `local.OldItem` null)
              (goto _label))))
        (:`NewEnumerator8`
          ;[1 1 1] Handle swapping weapons
          (`|ExecutionSequence`
            (:`then_0`
              (set `local.OrigLeftWeapon` _lefthandweapon))
            (:`then_1`
              (set `local.OrigRightWeapon` _righthandweapon))
            (:`then_2`
              (if (`|EnumEquality` (`/Game/Blueprint/Items/0_Item.WeaponHanded` (`local.NewItem`)) "NewEnumerator2")
                ;[1 1 1] If the new weapon is strictly two handed, remove both current weapons and equip new one
                (`|ExecutionSequence`
                  (:`then_0`
                    (bind _output_get_2 (set `local.OldItem` (`local.OrigRightWeapon`)))
                    (`self.UpdateEquimentSlot` _output_get_2 "NewEnumerator8" (`/Game/UMG/InventoryPanel.RightHand` _inventorypanel_2) (`local.NewItem`)))
                  (:`then_1`
                    (bind _output_get_3 (set `local.OtherOldItem` (`local.OrigLeftWeapon`)))
                    (`self.UpdateEquimentSlot` _output_get_3 "NewEnumerator7" _lefthand
                      (:`  `
                        (`/Game/UMG/ItemInInventory.UpdateSlot` _lefthand false null)))))
                (else
                  ;[1 1 1] New one handed - check for strict two handed in left hand, else replace either if the slot is free, or replace left
                  (`/Engine/EditorBlueprintResources/StandardMacros.IsValid` _origrightweapon
                    (:`Is Valid`
                      (if (`|EnumEquality` (`/Game/Blueprint/Items/0_Item.WeaponHanded` _origrightweapon_2) "NewEnumerator2")
                        (bind _output_get_4 (set `local.OldItem` _origrightweapon_2))
                        (`self.UpdateEquimentSlot` _output_get_4 "NewEnumerator8" _righthand (`local.NewItem`)
                          (:`  `
                            (`/Game/UMG/ItemInInventory.UpdateSlot` _lefthand_2 false null)))
                        (else
                          (`/Engine/EditorBlueprintResources/StandardMacros.IsValid` (`local.OrigLeftWeapon`)
                            (:`Is Valid`
                              (set `local.OldItem` _origrightweapon)
                              (`self.SetEquipmentSlot` _asmy_game_instance "NewEnumerator8" (`local.NewItem`) :!label _label_2)
                              (`/Game/UMG/ItemInInventory.UpdateSlot` _righthand true (`local.NewItem`)))
                            (:`Is Not Valid`
                              (set `local.OldItem` null)
                              (`self.SetEquipmentSlot` _asmy_game_instance "NewEnumerator7" (`local.NewItem`))
                              (`/Game/UMG/ItemInInventory.UpdateSlot` _lefthand_2 true (`local.NewItem`)))))))
                    (:`Is Not Valid`
                      (set `local.OldItem` null)
                      (goto _label_2))))))))
        (:`NewEnumerator9`
          (`KismetSystemLibrary.PrintString` "Cannot equip!" true true (struct :`R` 1.0 :`B` 0.024324 :`A` 1.0)))))
    (:`then_1`
      (return (`local.OldItem`) (`local.OtherOldItem`)))))

(fn `AddItemToStash`
  (params (Item :type "/Game/Blueprint/Items/0_Item Object Reference"))
  (returns (`Stored?` :type Boolean))
  (locals (NewItem :type "/Game/Blueprint/Items/0_Item Object Reference"))
  (`/Engine/EditorBlueprintResources/StandardMacros.IsValid` Item
    (:`Is Valid`
      (set `local.NewItem` Item)
      (for (_array_element _array_index) (`self.Stash`)
        (bind (_x _y _full_) (break `/Game/Blueprint/Structures/sStashSlot` _array_element))
        (if (not _full_)
          (bind _sstashslot (make `/Game/Blueprint/Structures/sStashSlot` _x _y true (`local.NewItem`)))
          (`KismetArrayLibrary.Array_Set` (`self.Stash`) _array_index _sstashslot)
          (bind _asin_game_controller (cast `/Game/Blueprint/InGameController` (`GameplayStatics.GetPlayerController` 0)))
          (`/Game/UMG/InventoryPanel.UpdateStashSlot` (`/Game/UMG/HUD.InventoryPanel` (`/Game/Blueprint/InGameController.HUD` _asin_game_controller)) _sstashslot)
          (return true)))
      (return false))))

(fn `AutoequipItem`
  (params (Item :type "/Game/Blueprint/Items/0_Item Object Reference"))
  (returns (Equipped :type Boolean))
  (locals (LocalEquipped :type Boolean) (LocalItem :type "/Game/Blueprint/Items/0_Item Object Reference"))
  (bind _output_get (set `local.LocalItem` Item))
  (switch `/Game/Blueprint/Enumerations/eItemTYpes` (`/Game/Blueprint/Items/0_Item.Type` _output_get)
    (:`NewEnumerator0`
      (`/Engine/EditorBlueprintResources/StandardMacros.IsValid` (`.Helmet_2_C9B9994541AFA5221E4C8D996C4FB8EC` (break `/Game/Blueprint/Structures/sCharacterEquipment` (`self.Equipment`)))
        (:`Is Valid`
          (set `local.LocalEquipped` false))
        (:`Is Not Valid`
          (set `local.LocalEquipped` true)
          (bind _structout (setmembers `/Game/Blueprint/Structures/sCharacterEquipment` :`StructRef` (make `/Game/Blueprint/Structures/sCharacterEquipment` (`local.LocalItem`))))
          (set `self.Equipment` _structout)))
      (return (`local.LocalEquipped`)))
    (:`NewEnumerator9`
      (set `local.LocalEquipped` false))))

(fn `ClearStashSlot`
  (params (SlotNumber :type Integer))
  (bind _stash (`self.Stash`))
  (bind (_x _y) (break `/Game/Blueprint/Structures/sStashSlot` (`|GetArrayItem` _stash SlotNumber)))
  (`KismetArrayLibrary.Array_Set` _stash SlotNumber (make `/Game/Blueprint/Structures/sStashSlot` _x _y)))

(fn `CreateNewCharacter`
  (params (NewCharacterName :type String))
  (returns (Success :type Boolean))
  (locals (NotFound :type Boolean :default true))
  (for _array_element (`self.ListOfCharacterSaves`)
    (if (`KismetStringLibrary.EqualEqual_StrStr` _array_element NewCharacterName)
      (set `local.NotFound` false)
      (break)))
  (if (`local.NotFound`)
    (`KismetArrayLibrary.Array_Add` (`self.ListOfCharacterSaves`) NewCharacterName)
    (`self.SaveCharacterList`))
  (return (`local.NotFound`)))

(fn `InitialiseStash`
  (locals (NewStashSlot :type "/Game/Blueprint/Structures/sStashSlot Structure"))
  (`KismetArrayLibrary.Array_Clear` (`self.Stash`))
  (for _index (range 40)
    (set `local.NewStashSlot` (make `/Game/Blueprint/Structures/sStashSlot` (mod _index 10) (/ _index 10)))
    (`KismetArrayLibrary.Array_Add` (`self.Stash`) (`local.NewStashSlot`))))

(fn `LoadCharacterList`
  (returns (Success :type Boolean))
  (locals (`LoadSuccessful?` :type Boolean))
  (bind _returnvalue (`GameplayStatics.DoesSaveGameExist` (`self.CharacterListSlotName`)))
  (if _returnvalue
    (bind _returnvalue_2 (`GameplayStatics.LoadGameFromSlot` (`self.CharacterListSlotName`)))
    (bind _aslist_of_characters (cast `/Game/Blueprint/ListOfCharacters` _returnvalue_2)
      (:`then`
        (set `self.ListOfCharacterSaves` (`/Game/Blueprint/ListOfCharacters.ListOfCharacters` _aslist_of_characters))
        (set `local.LoadSuccessful?` true))
      (:`CastFailed`
        _)))
  (return (`local.LoadSuccessful?`)))

(fn `RefreshStash`)

(fn `SaveCharacterList`
  (locals (LocalSaveFile :type "/Game/Blueprint/ListOfCharacters Object Reference"))
  (bind _returnvalue (`GameplayStatics.CreateSaveGameObject` "/Game/Blueprint/ListOfCharacters.ListOfCharacters_C"))
  (bind _output_get (set `local.LocalSaveFile` _returnvalue))
  (set `/Game/Blueprint/ListOfCharacters.ListOfCharacters` (`self.ListOfCharacterSaves`) _output_get)
  (`GameplayStatics.SaveGameToSlot` (`local.LocalSaveFile`) (`self.CharacterListSlotName`)))

(fn `SetEquipmentSlot`
  (params (EquipSlot :type "/Game/Blueprint/Enumerations/eEquipmentSlots Enum" :default "NewEnumerator0") (Item :type "/Game/Blueprint/Items/0_Item Object Reference"))
  (bind _equipment (`self.Equipment`))
  (switch `/Game/Blueprint/Enumerations/eEquipmentSlots` EquipSlot
    (:`NewEnumerator0`
      (bind _structout (setmembers `/Game/Blueprint/Structures/sCharacterEquipment` :`StructRef` _equipment :`Helmet` Item))
      (set `self.Equipment` _structout))
    (:`NewEnumerator1`
      (bind _structout_2 (setmembers `/Game/Blueprint/Structures/sCharacterEquipment` :`StructRef` _equipment :`Shoulders` Item))
      (set `self.Equipment` _structout_2))
    (:`NewEnumerator2`
      (bind _structout_3 (setmembers `/Game/Blueprint/Structures/sCharacterEquipment` :`StructRef` _equipment :`Chest` Item))
      (set `self.Equipment` _structout_3))
    (:`NewEnumerator3`
      (bind _structout_4 (setmembers `/Game/Blueprint/Structures/sCharacterEquipment` :`StructRef` _equipment :`Backpack` Item))
      (set `self.Equipment` _structout_4))
    (:`NewEnumerator4`
      (bind _structout_5 (setmembers `/Game/Blueprint/Structures/sCharacterEquipment` :`StructRef` _equipment :`Arms` Item))
      (set `self.Equipment` _structout_5))
    (:`NewEnumerator5`
      (bind _structout_6 (setmembers `/Game/Blueprint/Structures/sCharacterEquipment` :`StructRef` _equipment :`Belt` Item))
      (set `self.Equipment` _structout_6))
    (:`NewEnumerator6`
      (bind _structout_7 (setmembers `/Game/Blueprint/Structures/sCharacterEquipment` :`StructRef` _equipment :`Legs` Item))
      (set `self.Equipment` _structout_7))
    (:`NewEnumerator7`
      (bind _structout_8 (setmembers `/Game/Blueprint/Structures/sCharacterEquipment` :`StructRef` _equipment :`LeftHandWeapon` Item))
      (set `self.Equipment` _structout_8))
    (:`NewEnumerator8`
      (bind _structout_9 (setmembers `/Game/Blueprint/Structures/sCharacterEquipment` :`StructRef` _equipment :`RightHandWeapon` Item))
      (set `self.Equipment` _structout_9))
    (:`NewEnumerator9`
      (bind _structout_10 (setmembers `/Game/Blueprint/Structures/sCharacterEquipment` :`StructRef` _equipment :`Trinket1` Item))
      (set `self.Equipment` _structout_10))
    (:`NewEnumerator10`
      (bind _structout_11 (setmembers `/Game/Blueprint/Structures/sCharacterEquipment` :`StructRef` _equipment :`Trinket2` Item))
      (set `self.Equipment` _structout_11))))